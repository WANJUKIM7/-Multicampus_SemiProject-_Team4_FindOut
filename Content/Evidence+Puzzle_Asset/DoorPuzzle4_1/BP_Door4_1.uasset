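; BP_Door4_1 is a puzzle door actor that shows a four-digit password through four decal components, from Num1Left to Num4Right.
; The construction script calls ApplyNumber, which creates and caches a dynamic material instance per decal when none is valid, then sets its InputedNumber scalar from the matching InputPassword variable.
; The event graph holds only empty events, so the file has no runtime input, checking or opening logic.
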(event EventBeginPlay)

(event Collision|EventActorBeginOverlap
  (params (OtherActor :type Actor%20Object%20Reference)))

(event EventTick
  (params (DeltaSeconds :type Float%20%28single-precision%29)))

(fn ConstructionScript
  (CallFunction|ApplyNumber))

(fn ApplyNumber
  (bind _num1_left (Variables|Default|GetNum1_Left))
  (bind _num2 (Variables|Default|GetNum2))
  (bind _num3 (Variables|Default|GetNum3))
  (bind _num4_right (Variables|Default|GetNum4_Right))
  (Utilities|FlowControl|Sequence
    (:then_0
      ;[1 1 1] 1번쨰자리
      (Variables|Decal|GetMI_Door4_1Num1
        (:then
          _)
        (:else
          (bind _returnvalue (Rendering|Material|CreateDynamicMaterialInstance (Class|DecalComponent|GetDecalMaterial _num1_left) "None" "None" :!class /Script/Engine.KismetMaterialLibrary))
          (bind _output_get (Variables|Decal|SetMI_Door4_1Num1 _returnvalue))
          (Rendering|Components|Decal|SetDecalMaterial _num1_left _output_get)))
      (Rendering|Material|SetScalarParameterValue (Variables|Decal|GetMI_Door4_1Num1) "InputedNumber" (Variables|Default|GetInputPassword01) :!class /Script/Engine.MaterialInstanceDynamic))
    (:then_1
      ;[1 1 1] 2번쨰자리
      (Variables|Decal|GetMI_Door4_1Num2
        (:then
          _)
        (:else
          (bind _returnvalue_2 (Rendering|Material|CreateDynamicMaterialInstance (Class|DecalComponent|GetDecalMaterial _num2) "None" "None" :!class /Script/Engine.KismetMaterialLibrary))
          (bind _output_get_2 (Variables|Decal|SetMI_Door4_1Num2 _returnvalue_2))
          (Rendering|Components|Decal|SetDecalMaterial _num2 _output_get_2)))
      (Rendering|Material|SetScalarParameterValue (Variables|Decal|GetMI_Door4_1Num2) "InputedNumber" (Math|Conversions|ToFloat(Integer) (Variables|Default|GetInputPassword02)) :!class /Script/Engine.MaterialInstanceDynamic))
    (:then_2
      ;[1 1 1] 3번쨰자리
      (Variables|Decal|GetMI_Door4_1Num3
        (:then
          _)
        (:else
          (bind _returnvalue_3 (Rendering|Material|CreateDynamicMaterialInstance (Class|DecalComponent|GetDecalMaterial _num3) "None" "None" :!class /Script/Engine.KismetMaterialLibrary))
          (bind _output_get_3 (Variables|Decal|SetMI_Door4_1Num3 _returnvalue_3))
          (Rendering|Components|Decal|SetDecalMaterial _num3 _output_get_3)))
      (Rendering|Material|SetScalarParameterValue (Variables|Decal|GetMI_Door4_1Num3) "InputedNumber" (Math|Conversions|ToFloat(Integer) (Variables|Default|GetInputPassword03)) :!class /Script/Engine.MaterialInstanceDynamic))
    (:then_3
      ;[1 1 1] 4번쨰자리
      (Variables|Decal|GetMI_Door4_1Num4
        (:then
          _)
        (:else
          (bind _returnvalue_4 (Rendering|Material|CreateDynamicMaterialInstance (Class|DecalComponent|GetDecalMaterial _num4_right) "None" "None" :!class /Script/Engine.KismetMaterialLibrary))
          (bind _output_get_4 (Variables|Decal|SetMI_Door4_1Num4 _returnvalue_4))
          (Rendering|Components|Decal|SetDecalMaterial _num4_right _output_get_4)))
      (Rendering|Material|SetScalarParameterValue (Variables|Decal|GetMI_Door4_1Num4) "InputedNumber" (Math|Conversions|ToFloat(Integer) (Variables|Default|GetInputPassword04)) :!class /Script/Engine.MaterialInstanceDynamic))))