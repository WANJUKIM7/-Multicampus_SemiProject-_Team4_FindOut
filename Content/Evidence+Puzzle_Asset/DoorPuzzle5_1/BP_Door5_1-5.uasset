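; Keypad door puzzle where the player zooms in via an overlap volume and clicks digit, back and enter buttons to enter a four-digit code.
; Input builds a Passwords array, shown right-aligned on four decals through lazily created dynamic material instances.
; Enter compares it to the InputPassword values, then either zooms out, fires the Trigger and marks it solved, or resets and briefly locks input.
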(event OnComponentBeginOverlap(ZoomCollision)
  (params (OverlappedComponent :type Primitive%20Component%20Object%20Reference) (OtherActor :type Actor%20Object%20Reference) (OtherComp :type Primitive%20Component%20Object%20Reference) (OtherBodyIndex :type Integer) (bFromSweep :type Boolean) (SweepResult :type Hit%20Result%20Structure%20%28by%20ref%29))
  ;[1 1 1] 카메라 줌 오버랩
  (CallFunction|BeginOverlapPuzzle OtherActor self (Variables|Default|GetCamera)))

(event OnComponentEndOverlap(ZoomCollision)
  (params (OverlappedComponent :type Primitive%20Component%20Object%20Reference) (OtherActor :type Actor%20Object%20Reference) (OtherComp :type Primitive%20Component%20Object%20Reference) (OtherBodyIndex :type Integer))
  ;[1 1 1] 카메라 줌 오버랩
  (CallFunction|EndOverlapPuzzle OtherActor))

(event OnClicked(Keypad_9)
  (params (TouchedComponent :type Primitive%20Component%20Object%20Reference) (ButtonPressed :type Key%20Structure :default "None"))
  ;[1 1 1] 키패드 클릭
  (if (Variables|Default|GetCanClick?)
    (Utilities|Array|Add (Variables|Default|GetPasswords) 9)
    (CallFunction|ApplyNumber)))

(event OnClicked(Keypad_0)
  (params (TouchedComponent :type Primitive%20Component%20Object%20Reference) (ButtonPressed :type Key%20Structure :default "None"))
  ;[1 1 1] 키패드 클릭
  (if (Variables|Default|GetCanClick?)
    (Utilities|Array|Add (Variables|Default|GetPasswords) 0)
    (CallFunction|ApplyNumber)))

(event OnClicked(Keypad_Enter)
  (params (TouchedComponent :type Primitive%20Component%20Object%20Reference) (ButtonPressed :type Key%20Structure :default "None"))
  ;[1 1 1] 키패드 클릭
  (if (Variables|Default|GetCanClick?)
    (CallFunction|CheckAnswer)))

(event OnClicked(Keypad_Back)
  (params (TouchedComponent :type Primitive%20Component%20Object%20Reference) (ButtonPressed :type Key%20Structure :default "None"))
  ;[1 1 1] 키패드 클릭
  (if (Variables|Default|GetCanClick?)
    (CallFunction|Back)
    (CallFunction|ApplyNumber)))

(event OnClicked(Keypad_2)
  (params (TouchedComponent :type Primitive%20Component%20Object%20Reference) (ButtonPressed :type Key%20Structure :default "None"))
  ;[1 1 1] 키패드 클릭
  (if (Variables|Default|GetCanClick?)
    (Utilities|Array|Add (Variables|Default|GetPasswords) 2)
    (CallFunction|ApplyNumber)))

(event OnClicked(Keypad_3)
  (params (TouchedComponent :type Primitive%20Component%20Object%20Reference) (ButtonPressed :type Key%20Structure :default "None"))
  ;[1 1 1] 키패드 클릭
  (if (Variables|Default|GetCanClick?)
    (Utilities|Array|Add (Variables|Default|GetPasswords) 3)
    (CallFunction|ApplyNumber)))

(event OnClicked(Keypad_1)
  (params (TouchedComponent :type Primitive%20Component%20Object%20Reference) (ButtonPressed :type Key%20Structure :default "None"))
  ;[1 1 1] 키패드 클릭
  (if (Variables|Default|GetCanClick?)
    (Utilities|Array|Add (Variables|Default|GetPasswords) 1)
    (CallFunction|ApplyNumber)))

(event OnClicked(Keypad_4)
  (params (TouchedComponent :type Primitive%20Component%20Object%20Reference) (ButtonPressed :type Key%20Structure :default "None"))
  ;[1 1 1] 키패드 클릭
  (if (Variables|Default|GetCanClick?)
    (Utilities|Array|Add (Variables|Default|GetPasswords) 4)
    (CallFunction|ApplyNumber)))

(event OnClicked(Keypad_5)
  (params (TouchedComponent :type Primitive%20Component%20Object%20Reference) (ButtonPressed :type Key%20Structure :default "None"))
  ;[1 1 1] 키패드 클릭
  (if (Variables|Default|GetCanClick?)
    (Utilities|Array|Add (Variables|Default|GetPasswords) 5)
    (CallFunction|ApplyNumber)))

(event OnClicked(Keypad_6)
  (params (TouchedComponent :type Primitive%20Component%20Object%20Reference) (ButtonPressed :type Key%20Structure :default "None"))
  ;[1 1 1] 키패드 클릭
  (if (Variables|Default|GetCanClick?)
    (Utilities|Array|Add (Variables|Default|GetPasswords) 6)
    (CallFunction|ApplyNumber)))

(event OnClicked(Keypad_7)
  (params (TouchedComponent :type Primitive%20Component%20Object%20Reference) (ButtonPressed :type Key%20Structure :default "None"))
  ;[1 1 1] 키패드 클릭
  (if (Variables|Default|GetCanClick?)
    (Utilities|Array|Add (Variables|Default|GetPasswords) 7)
    (CallFunction|ApplyNumber)))

(event OnClicked(Keypad_8)
  (params (TouchedComponent :type Primitive%20Component%20Object%20Reference) (ButtonPressed :type Key%20Structure :default "None"))
  ;[1 1 1] 키패드 클릭
  (if (Variables|Default|GetCanClick?)
    (Utilities|Array|Add (Variables|Default|GetPasswords) 8)
    (CallFunction|ApplyNumber)))

(event Custom|CheckingAnswer
  ;[1 1 1] Checking Answer
  (Input|DisableInput (Game|GetPlayerCharacter 0) 0)
  (Variables|Default|SetCanClick? false)
  (Utilities|FlowControl|Delay 2.0)
  (Input|EnableInput (Game|GetPlayerCharacter 0) 0)
  (Variables|Default|SetCanClick? true))

(event Custom|Reset
  ;[1 1 1] 초기화
  (Utilities|Array|Clear (Variables|Default|GetPasswords))
  (bind _mi_door4_1num1 (Variables|Decal|GetMI_Door4_1Num1)
    (:then
      (Rendering|Material|SetScalarParameterValue _mi_door4_1num1 "InputedNumber" 0.0 :!class /Script/Engine.MaterialInstanceDynamic))
    (:else
      _))
  (bind _mi_door4_1num2 (Variables|Decal|GetMI_Door4_1Num2)
    (:then
      (Rendering|Material|SetScalarParameterValue _mi_door4_1num2 "InputedNumber" 0.0 :!class /Script/Engine.MaterialInstanceDynamic))
    (:else
      _))
  (bind _mi_door4_1num3 (Variables|Decal|GetMI_Door4_1Num3)
    (:then
      (Rendering|Material|SetScalarParameterValue _mi_door4_1num3 "InputedNumber" 0.0 :!class /Script/Engine.MaterialInstanceDynamic))
    (:else
      _))
  (bind _mi_door4_1num4 (Variables|Decal|GetMI_Door4_1Num4)
    (:then
      (Rendering|Material|SetScalarParameterValue _mi_door4_1num4 "InputedNumber" 0.0 :!class /Script/Engine.MaterialInstanceDynamic))
    (:else)))

(event Custom|SetFourthNumber
  (bind _num4 (Variables|Default|GetNum4))
  (bind _passwords (Variables|Default|GetPasswords))
  ;[1 1 1] SetNumber
  (Variables|Decal|GetMI_Door4_1Num4
    (:then
      _)
    (:else
      (bind _returnvalue (Rendering|Material|CreateDynamicMaterialInstance (Class|DecalComponent|GetDecalMaterial _num4) "None" "None" :!class /Script/Engine.KismetMaterialLibrary))
      (bind _output_get (Variables|Decal|SetMI_Door4_1Num4 _returnvalue))
      (Rendering|Components|Decal|SetDecalMaterial _num4 _output_get)))
  (Rendering|Material|SetScalarParameterValue (Variables|Decal|GetMI_Door4_1Num4) "InputedNumber" (Math|Conversions|ToFloat(Integer) (Utilities|Array|Get(acopy) _passwords (- (Utilities|Array|Length _passwords) 1))) :!class /Script/Engine.MaterialInstanceDynamic))

(event Custom|SetThirdNumber
  (bind _passwords (Variables|Default|GetPasswords))
  (bind _num3 (Variables|Default|GetNum3))
  ;[1 1 1] SetNumber
  (Variables|Decal|GetMI_Door4_1Num3
    (:then
      _)
    (:else
      (bind _returnvalue (Rendering|Material|CreateDynamicMaterialInstance (Class|DecalComponent|GetDecalMaterial _num3) "None" "None" :!class /Script/Engine.KismetMaterialLibrary))
      (bind _output_get (Variables|Decal|SetMI_Door4_1Num3 _returnvalue))
      (Rendering|Components|Decal|SetDecalMaterial _num3 _output_get)))
  (Rendering|Material|SetScalarParameterValue (Variables|Decal|GetMI_Door4_1Num3) "InputedNumber" (Math|Conversions|ToFloat(Integer) (Utilities|Array|Get(acopy) _passwords (- (Utilities|Array|Length _passwords) 2))) :!class /Script/Engine.MaterialInstanceDynamic))

(event Custom|SetSecondNumber
  (bind _num2 (Variables|Default|GetNum2))
  (bind _passwords (Variables|Default|GetPasswords))
  ;[1 1 1] SetNumber
  (Variables|Decal|GetMI_Door4_1Num2
    (:then
      _)
    (:else
      (bind _returnvalue (Rendering|Material|CreateDynamicMaterialInstance (Class|DecalComponent|GetDecalMaterial _num2) "None" "None" :!class /Script/Engine.KismetMaterialLibrary))
      (bind _output_get (Variables|Decal|SetMI_Door4_1Num2 _returnvalue))
      (Rendering|Components|Decal|SetDecalMaterial _num2 _output_get)))
  (Rendering|Material|SetScalarParameterValue (Variables|Decal|GetMI_Door4_1Num2) "InputedNumber" (Math|Conversions|ToFloat(Integer) (Utilities|Array|Get(acopy) _passwords (- (Utilities|Array|Length _passwords) 3))) :!class /Script/Engine.MaterialInstanceDynamic))

(event Custom|SetFirstNumber
  (bind _num1 (Variables|Default|GetNum1))
  (bind _passwords (Variables|Default|GetPasswords))
  ;[1 1 1] SetNumber
  (Variables|Decal|GetMI_Door4_1Num1
    (:then
      _)
    (:else
      (bind _returnvalue (Rendering|Material|CreateDynamicMaterialInstance (Class|DecalComponent|GetDecalMaterial _num1) "None" "None" :!class /Script/Engine.KismetMaterialLibrary))
      (bind _output_get (Variables|Decal|SetMI_Door4_1Num1 _returnvalue))
      (Rendering|Components|Decal|SetDecalMaterial _num1 _output_get)))
  (Rendering|Material|SetScalarParameterValue (Variables|Decal|GetMI_Door4_1Num1) "InputedNumber" (Math|Conversions|ToFloat(Integer) (Utilities|Array|Get(acopy) _passwords (- (Utilities|Array|Length _passwords) 4))) :!class /Script/Engine.MaterialInstanceDynamic))

(event EventBeginPlay
  ;[1 1 1] BeginPlay
  (Variables|Default|SetDisplayDescription "Press Button")
  (Input|DisableInput (Game|GetPlayerController 0)))

(event EventZoomonEvent
  (params (PlayerCharacter :type BP%20First%20Person%20Character%20Object%20Reference))
  ;[1 1 1] Zoom on / out 시 이벤트
  (|CallParentFunction PlayerCharacter)
  (Variables|Default|SetCanClick? true))

(event EventZoomOutEvent
  ;[1 1 1] Zoom on / out 시 이벤트
  (|CallParentFunction)
  (Variables|Default|SetCanClick? false))

(event EventInterfaceToggleFocus
  (params (Focus :type Boolean))
  ;[1 1 1] Outline
  (Rendering|SetRenderCustomDepth (Variables|Default|GetDoorLock) Focus))

(event Input|KeyboardEvents|3
  (params (Key :type Key%20Structure :default "None"))
  ;[1 1 1] Test
)

(fn ConstructionScript
  (CallFunction|ApplyNumber))

(fn ApplyNumber
  (switch int (Utilities|Array|Length (Variables|Default|GetPasswords))
    (:1
      (CallFunction|SetFourthNumber))
    (:2
      (CallFunction|SetThirdNumber)
      (CallFunction|SetFourthNumber))
    (:3
      (CallFunction|SetSecondNumber)
      (CallFunction|SetThirdNumber)
      (CallFunction|SetFourthNumber))
    (:4
      (CallFunction|SetFirstNumber)
      (CallFunction|SetSecondNumber)
      (CallFunction|SetThirdNumber)
      (CallFunction|SetFourthNumber))))

(fn CheckAnswer
  ;[1 1 1] 정답 확인
  (if (== (Utilities|Array|Get(acopy) (Variables|Default|GetPasswords)) (Variables|Default|GetInputPassword01))
    (if (== (Utilities|Array|Get(acopy) (Variables|Default|GetPasswords) 1) (Variables|Default|GetInputPassword02))
      (if (== (Utilities|Array|Get(acopy) (Variables|Default|GetPasswords) 2) (Variables|Default|GetInputPassword03))
        (if (== (Utilities|Array|Get(acopy) (Variables|Default|GetPasswords) 3) (Variables|Default|GetInputPassword04))
          (CallFunction|ZoomOutPuzzle self)
          (Default|Trigger (Variables|Default|GetTrigger))
          (Variables|Default|SetTags (Variables|Default|Get태그))
          (Variables|Default|SetSolved? true)
          (else
            (CallFunction|Reset :!label _label)
            (CallFunction|CheckingAnswer)))
        (else
          (goto _label)))
      (else
        (goto _label)))
    (else
      (goto _label))))

(fn Back
  (bind _num1 (Variables|Default|GetNum1))
  (bind _num4 (Variables|Default|GetNum4))
  (bind _num2 (Variables|Default|GetNum2))
  (bind _num3 (Variables|Default|GetNum3))
  (bind _passwords (Variables|Default|GetPasswords))
  (bind _returnvalue (Utilities|Array|Length _passwords))
  (bind _returnvalue_2 (- _returnvalue 1))
  (if (>= _returnvalue_2 0)
    (Utilities|Array|RemoveIndex _passwords _returnvalue_2)
    (switch int _returnvalue
      (:Default
        (Development|PrintString "Back Default"))
      (:0
        (Variables|Decal|GetMI_Door4_1Num4
          (:then
            _)
          (:else
            (bind _returnvalue_3 (Rendering|Material|CreateDynamicMaterialInstance (Class|DecalComponent|GetDecalMaterial _num4) "None" "None" :!class /Script/Engine.KismetMaterialLibrary))
            (bind _output_get (Variables|Decal|SetMI_Door4_1Num4 _returnvalue_3))
            (Rendering|Components|Decal|SetDecalMaterial _num4 _output_get)))
        (Rendering|Material|SetScalarParameterValue (Variables|Decal|GetMI_Door4_1Num4) "InputedNumber" 0.0 :!class /Script/Engine.MaterialInstanceDynamic))
      (:1
        (Variables|Decal|GetMI_Door4_1Num3
          (:then
            _)
          (:else
            (bind _returnvalue_4 (Rendering|Material|CreateDynamicMaterialInstance (Class|DecalComponent|GetDecalMaterial _num3) "None" "None" :!class /Script/Engine.KismetMaterialLibrary))
            (bind _output_get_2 (Variables|Decal|SetMI_Door4_1Num3 _returnvalue_4))
            (Rendering|Components|Decal|SetDecalMaterial _num3 _output_get_2)))
        (Rendering|Material|SetScalarParameterValue (Variables|Decal|GetMI_Door4_1Num3) "InputedNumber" 0.0 :!class /Script/Engine.MaterialInstanceDynamic))
      (:2
        (Variables|Decal|GetMI_Door4_1Num2
          (:then
            _)
          (:else
            (bind _returnvalue_5 (Rendering|Material|CreateDynamicMaterialInstance (Class|DecalComponent|GetDecalMaterial _num2) "None" "None" :!class /Script/Engine.KismetMaterialLibrary))
            (bind _output_get_3 (Variables|Decal|SetMI_Door4_1Num2 _returnvalue_5))
            (Rendering|Components|Decal|SetDecalMaterial _num2 _output_get_3)))
        (Rendering|Material|SetScalarParameterValue (Variables|Decal|GetMI_Door4_1Num2) "InputedNumber" 0.0 :!class /Script/Engine.MaterialInstanceDynamic))
      (:3
        (Variables|Decal|GetMI_Door4_1Num1
          (:then
            _)
          (:else
            (bind _returnvalue_6 (Rendering|Material|CreateDynamicMaterialInstance (Class|DecalComponent|GetDecalMaterial _num1) "None" "None" :!class /Script/Engine.KismetMaterialLibrary))
            (bind _output_get_4 (Variables|Decal|SetMI_Door4_1Num1 _returnvalue_6))
            (Rendering|Components|Decal|SetDecalMaterial _num1 _output_get_4)))
        (Rendering|Material|SetScalarParameterValue (Variables|Decal|GetMI_Door4_1Num1) "InputedNumber" 0.0 :!class /Script/Engine.MaterialInstanceDynamic)))))

(fn SetDisabled
  (Input|DisableInput (Game|GetPlayerController 0))
  (Collision|SetCollisionEnabled (Variables|Default|GetKeypad_0) "NoCollision")
  (Collision|SetCollisionEnabled (Variables|Default|GetKeypad_1) "NoCollision")
  (Collision|SetCollisionEnabled (Variables|Default|GetKeypad_2) "NoCollision")
  (Collision|SetCollisionEnabled (Variables|Default|GetKeypad_3) "NoCollision")
  (Collision|SetCollisionEnabled (Variables|Default|GetKeypad_4) "NoCollision")
  (Collision|SetCollisionEnabled (Variables|Default|GetKeypad_5) "NoCollision")
  (Collision|SetCollisionEnabled (Variables|Default|GetKeypad_6) "NoCollision")
  (Collision|SetCollisionEnabled (Variables|Default|GetKeypad_7) "NoCollision")
  (Collision|SetCollisionEnabled (Variables|Default|GetKeypad_8) "NoCollision")
  (Collision|SetCollisionEnabled (Variables|Default|GetKeypad_9) "NoCollision")
  (Collision|SetCollisionEnabled (Variables|Default|GetKeypad_Back) "NoCollision")
  (Collision|SetCollisionEnabled (Variables|Default|GetKeypad_Enter) "NoCollision"))