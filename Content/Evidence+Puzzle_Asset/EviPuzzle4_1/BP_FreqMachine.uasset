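; BP_FreqMachine is a frequency-machine puzzle actor with a mouse-draggable dial and a screen material switchable between on and noised.
; Overlapping its collision box calls the puzzle begin/end functions, passing its camera on entry.
; While dragging, a cursor trace against MouseCollisionBox sets rotation velocities from the dial-relative hit point, turning mouse movement into rotation.
; ScreenOn checks for a narrow target angle, but its branch is empty.
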(event OnComponentBeginOverlap(CollisionBox)
  (params (OverlappedComponent :type Primitive%20Component%20Object%20Reference) (OtherActor :type Actor%20Object%20Reference) (OtherComp :type Primitive%20Component%20Object%20Reference) (OtherBodyIndex :type Integer) (bFromSweep :type Boolean) (SweepResult :type Hit%20Result%20Structure%20%28by%20ref%29))
  ;[1 1 1] 카메라 줌 오버랩
  (CallFunction|BeginOverlapPuzzle OtherActor self (Variables|Default|GetCamera)))

(event OnComponentEndOverlap(CollisionBox)
  (params (OverlappedComponent :type Primitive%20Component%20Object%20Reference) (OtherActor :type Actor%20Object%20Reference) (OtherComp :type Primitive%20Component%20Object%20Reference) (OtherBodyIndex :type Integer))
  ;[1 1 1] 카메라 줌 오버랩
  (CallFunction|EndOverlapPuzzle OtherActor))

(event OnClicked(Dial)
  (params (TouchedComponent :type Primitive%20Component%20Object%20Reference) (ButtonPressed :type Key%20Structure :default "None"))
  ;[1 1 1] 다이얼 클릭시
  (Variables|Default|SetClickedDial? true)
  (Collision|SetCollisionEnabled (Variables|Default|GetDial) "NoCollision"))

(event EventTick
  (params (DeltaSeconds :type Float%20%28single-precision%29))
  ;[1 1 1] Event Tick
  (if (Variables|Default|GetClickedDial?)
    (CallFunction|SetRotateVelocity)
    (CallFunction|Rotate DeltaSeconds)
    (CallFunction|Screenon)))

(event EventBeginPlay
  ;[1 1 1] BeginPlay
)

(event Input|MouseEvents|LeftMouseButton
  (params (Key :type Key%20Structure :default "None"))
  ;[1 1 1] 다이얼 클릭시
  (:Released
    (Variables|Default|SetClickedDial? false)
    (Collision|SetCollisionEnabled (Variables|Default|GetDial) "QueryAndPhysics")))

(fn ConstructionScript
  (Rendering|Material|SetScalarParameterValueonMaterials (Variables|Default|GetMainScreen) "0=On_1=Noised" (Variables|Default|Get0=On~1=Noised)))

(fn Rotate
  (params (Delta :type Float%20%28double-precision%29))
  (bind _returnvalue (Game|GetPlayerController 0))
  (bind _rotateyvelocity (Variables|Default|GetRotateYVelocity))
  (bind _rotatexvelocity (Variables|Default|GetRotateXVelocity))
  (bind (_deltax _deltay) (Class|PlayerController|GetInputMouseDelta _returnvalue))
  (bind _returnvalue_2 (* _deltay Delta))
  (bind _returnvalue_3 (* _deltax Delta))
  (bind _returnvalue_4 (* _returnvalue_2 _rotateyvelocity))
  (bind _returnvalue_5 (* _returnvalue_3 _rotatexvelocity))
  (bind _returnvalue_6 (* _returnvalue_5 -1.0))
  (bind _returnvalue_7 (+ _returnvalue_6 _returnvalue_4))
  (Transformation|AddLocalRotation (Variables|Default|GetDial) (Math|Rotator|MakeRotator 0.0 _returnvalue_7 0.0) false false)
  ;[1 1 1] Set RotationValue
  (bind _output_get (Variables|Default|SetRotationValue (+ (Variables|Default|GetRotationValue) _returnvalue_7)))
  (if (> _output_get 3.6e+02)
    (Variables|Default|SetRotationValue (- _output_get 3.6e+02))
    (elif (< _output_get 0.0)
      (Variables|Default|SetRotationValue (+ _output_get 3.6e+02)))))

(fn SetRotateVelocity
  (bind _returnvalue (Game|GetPlayerController 0))
  (bind _dial (Variables|Default|GetDial))
  (bind _returnvalue_2 (Components|GetOwner _dial))
  (bind (_worldlocation _worlddirection) (Game|Player|ConvertMouseLocationToWorldSpace _returnvalue))
  (bind _returnvalue_3 (Transformation|GetActorTransform _returnvalue_2))
  (bind _outhit (Collision|LineTraceByChannel _worldlocation (+ _worldlocation (* _worlddirection (Variables|Default|GetLineTraceValue))) "TraceTypeQuery1" false 0 "None" false "(R=1.000000,G=0.000000,B=0.000000,A=1.000000)" "(R=0.000000,G=1.000000,B=0.000000,A=1.000000)" 1e+01))
  (if (== (.HitComponent (Collision|BreakHitResult _outhit)) (Variables|Default|GetMouseCollisionBox))
    (bind _output_get (Variables|Default|SetMouseRelativeLocation (- (Math|Transform|InverseTransformLocation _returnvalue_3 (.ImpactPoint (Collision|BreakHitResult _outhit))) (Math|Transform|InverseTransformLocation _returnvalue_3 (Transformation|GetWorldLocation (Variables|Default|GetDial))))))
    (Variables|Default|SetRotateXVelocity (* (.z _output_get) 3e+01))
    (Variables|Default|SetRotateYVelocity (* (.x _output_get) 3e+01))
    (else
      (Variables|Default|SetClickedDial? false))))

(fn Screenon
  (bind _rotationvalue (Variables|Default|GetRotationValue))
  (if (and (> _rotationvalue 1.8e+02) (< _rotationvalue 185.0))
    _))