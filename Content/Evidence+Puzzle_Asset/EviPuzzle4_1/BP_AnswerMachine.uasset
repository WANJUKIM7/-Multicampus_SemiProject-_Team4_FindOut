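; BP_AnswerMachine is an evidence puzzle: a four-by-four button panel where the player must press the correct combination, with camera zoom handled through overlap on ZoomCollision.
; Each click calls ButtonPress, which toggles that button in or out, updates ButtonPressed and Answer, then runs CheckAnswer.
; Exactly three correct buttons, in any order, fire Trigger, set Tags and zoom out.
; CheckPressed, a per-row test, is unused; key 3 prints Answer for debugging.
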(event OnComponentBeginOverlap(ZoomCollision)
  (params (OverlappedComponent :type Primitive%20Component%20Object%20Reference) (OtherActor :type Actor%20Object%20Reference) (OtherComp :type Primitive%20Component%20Object%20Reference) (OtherBodyIndex :type Integer) (bFromSweep :type Boolean) (SweepResult :type Hit%20Result%20Structure%20%28by%20ref%29))
  ;[1 1 1] 카메라 줌 오버랩
  (CallFunction|BeginOverlapPuzzle OtherActor self (Variables|Default|GetCamera)))

(event OnComponentEndOverlap(ZoomCollision)
  (params (OverlappedComponent :type Primitive%20Component%20Object%20Reference) (OtherActor :type Actor%20Object%20Reference) (OtherComp :type Primitive%20Component%20Object%20Reference) (OtherBodyIndex :type Integer))
  ;[1 1 1] 카메라 줌 오버랩
  (CallFunction|EndOverlapPuzzle OtherActor))

(event OnClicked(Button2_1)
  (params (TouchedComponent :type Primitive%20Component%20Object%20Reference) (ButtonPressed :type Key%20Structure :default "None"))
  ;[1 1 1] 클릭 이벤트
  (CallFunction|ButtonPress TouchedComponent 7 (Variables|Default|GetButton2_1)))

(event OnClicked(Button2_2)
  (params (TouchedComponent :type Primitive%20Component%20Object%20Reference) (ButtonPressed :type Key%20Structure :default "None"))
  ;[1 1 1] 클릭 이벤트
  (CallFunction|ButtonPress TouchedComponent 6 (Variables|Default|GetButton2_2)))

(event OnClicked(Button2_3)
  (params (TouchedComponent :type Primitive%20Component%20Object%20Reference) (ButtonPressed :type Key%20Structure :default "None"))
  ;[1 1 1] 클릭 이벤트
  (CallFunction|ButtonPress TouchedComponent 5 (Variables|Default|GetButton2_3)))

(event OnClicked(Button2_4)
  (params (TouchedComponent :type Primitive%20Component%20Object%20Reference) (ButtonPressed :type Key%20Structure :default "None"))
  ;[1 1 1] 클릭 이벤트
  (CallFunction|ButtonPress TouchedComponent 4 (Variables|Default|GetButton2_4)))

(event OnClicked(Button1_1)
  (params (TouchedComponent :type Primitive%20Component%20Object%20Reference) (ButtonPressed :type Key%20Structure :default "None"))
  ;[1 1 1] 클릭 이벤트
  (CallFunction|ButtonPress TouchedComponent 3 (Variables|Default|GetButton1_1)))

(event OnClicked(Button1_2)
  (params (TouchedComponent :type Primitive%20Component%20Object%20Reference) (ButtonPressed :type Key%20Structure :default "None"))
  ;[1 1 1] 클릭 이벤트
  (CallFunction|ButtonPress TouchedComponent 2 (Variables|Default|GetButton1_2)))

(event OnClicked(Button1_3)
  (params (TouchedComponent :type Primitive%20Component%20Object%20Reference) (ButtonPressed :type Key%20Structure :default "None"))
  ;[1 1 1] 클릭 이벤트
  (CallFunction|ButtonPress TouchedComponent 1 (Variables|Default|GetButton1_3)))

(event OnClicked(Button1_4)
  (params (TouchedComponent :type Primitive%20Component%20Object%20Reference) (ButtonPressed :type Key%20Structure :default "None"))
  ;[1 1 1] 클릭 이벤트
  (CallFunction|ButtonPress TouchedComponent 0 (Variables|Default|GetButton1_4)))

(event OnClicked(Button4_1)
  (params (TouchedComponent :type Primitive%20Component%20Object%20Reference) (ButtonPressed :type Key%20Structure :default "None"))
  ;[1 1 1] 클릭 이벤트
  (CallFunction|ButtonPress TouchedComponent 15 (Variables|Default|GetButton4_1)))

(event OnClicked(Button4_2)
  (params (TouchedComponent :type Primitive%20Component%20Object%20Reference) (ButtonPressed :type Key%20Structure :default "None"))
  ;[1 1 1] 클릭 이벤트
  (CallFunction|ButtonPress TouchedComponent 14 (Variables|Default|GetButton4_2)))

(event OnClicked(Button4_3)
  (params (TouchedComponent :type Primitive%20Component%20Object%20Reference) (ButtonPressed :type Key%20Structure :default "None"))
  ;[1 1 1] 클릭 이벤트
  (CallFunction|ButtonPress TouchedComponent 13 (Variables|Default|GetButton4_3)))

(event OnClicked(Button4_4)
  (params (TouchedComponent :type Primitive%20Component%20Object%20Reference) (ButtonPressed :type Key%20Structure :default "None"))
  ;[1 1 1] 클릭 이벤트
  (CallFunction|ButtonPress TouchedComponent 12 (Variables|Default|GetButton4_4)))

(event OnClicked(Button3_1)
  (params (TouchedComponent :type Primitive%20Component%20Object%20Reference) (ButtonPressed :type Key%20Structure :default "None"))
  ;[1 1 1] 클릭 이벤트
  (CallFunction|ButtonPress TouchedComponent 11 (Variables|Default|GetButton3_1)))

(event OnClicked(Button3_2)
  (params (TouchedComponent :type Primitive%20Component%20Object%20Reference) (ButtonPressed :type Key%20Structure :default "None"))
  ;[1 1 1] 클릭 이벤트
  (CallFunction|ButtonPress TouchedComponent 10 (Variables|Default|GetButton3_2)))

(event OnClicked(Button3_3)
  (params (TouchedComponent :type Primitive%20Component%20Object%20Reference) (ButtonPressed :type Key%20Structure :default "None"))
  ;[1 1 1] 클릭 이벤트
  (CallFunction|ButtonPress TouchedComponent 9 (Variables|Default|GetButton3_3)))

(event OnClicked(Button3_4)
  (params (TouchedComponent :type Primitive%20Component%20Object%20Reference) (ButtonPressed :type Key%20Structure :default "None"))
  ;[1 1 1] 클릭 이벤트
  (CallFunction|ButtonPress TouchedComponent 8 (Variables|Default|GetButton3_4)))

(event EventBeginPlay
  ;[1 1 1] BeginPlay
  (Variables|Default|SetDisplayDescription "Press button"))

(event Input|KeyboardEvents|3
  (params (Key :type Key%20Structure :default "None"))
  ;[1 1 1] Test
  (:Pressed
    (for (_array_element _array_index) (Variables|Default|GetAnswer)
      (Development|PrintText (Utilities|Text|FormatText "BP_AnswerMachine1 : {a}, {b}" _array_index (Utilities|GetDisplayName _array_element))))))

(fn ConstructionScript)

(fn ButtonPress
  (params (TouchedComponent :type Primitive%20Component%20Object%20Reference) (Index :type Integer) (SelectedStaticMeshComponent :type Static%20Mesh%20Component%20Object%20Reference))
  (bind _relativelocation (Variables|/Script/Engine.SceneComponent|GetRelativeLocation TouchedComponent))
  (if (Utilities|Array|Get(acopy) (Variables|Default|GetButtonPressed) Index)
    (Transformation|SetRelativeLocation TouchedComponent (+ _relativelocation "0.000000,2.000000,0.000000") false false)
    (Utilities|Array|SetArrayElem (Variables|Default|GetButtonPressed) Index false)
    (Utilities|Array|RemoveItem (Variables|Default|GetAnswer) SelectedStaticMeshComponent)
    (else
      (Transformation|SetRelativeLocation TouchedComponent (+ _relativelocation "0.000000,-2.000000,0.000000") false false)
      (Utilities|Array|SetArrayElem (Variables|Default|GetButtonPressed) Index true)
      (Utilities|Array|Add (Variables|Default|GetAnswer) SelectedStaticMeshComponent)))
  (CallFunction|CheckAnswer))

(fn CheckPressed
  (params (Index :type Integer))
  (switch int (/ Index 4)
    (:0
      (for (_array_element _array_index) (Variables|Default|GetButtonPressed)
        (if (== (/ _array_index 4) 0)
          (if _array_element
            (return true))))
      (return false))
    (:1
      (for (_array_element_2 _array_index_2) (Variables|Default|GetButtonPressed)
        (if (== (/ _array_index_2 4) 1)
          (if _array_element_2
            (return true))))
      (return false))
    (:2
      (for (_array_element_3 _array_index_3) (Variables|Default|GetButtonPressed)
        (if (== (/ _array_index_3 4) 2)
          (if _array_element_3
            (return true))))
      (return false))
    (:3
      (for (_array_element_4 _array_index_4) (Variables|Default|GetButtonPressed)
        (if (== (/ _array_index_4 4) 3)
          (if _array_element_4
            (return true))))
      (return false))))

(fn CheckAnswer
  (if (== (Utilities|Array|Length (Variables|Default|GetAnswer)) 3)
    (if (>= (Utilities|Array|FindItem (Variables|Default|GetAnswer) (Variables|Default|GetButton2_2)) 0)
      (if (>= (Utilities|Array|FindItem (Variables|Default|GetAnswer) (Variables|Default|GetButton3_1)) 0)
        (if (>= (Utilities|Array|FindItem (Variables|Default|GetAnswer) (Variables|Default|GetButton4_3)) 0)
          (Default|Trigger (Variables|Default|GetTrigger))
          (Variables|Default|SetTags (Variables|Default|Get태그))
          (CallFunction|ZoomOutPuzzle self))))))