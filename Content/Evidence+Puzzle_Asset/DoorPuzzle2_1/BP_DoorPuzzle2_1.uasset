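; BP_DoorPuzzle2_1 is a door puzzle with a rotating two-arrow button that toggles circular parts on and off.
; An overlap zone registers it with the player for camera zoom, and input acts only while zoomed into this puzzle.
; D and A rotate the button through timelines, and arrow collisions track the two selected parts.
; Left click swaps both parts' On/Off materials by comparing material names; CheckAnswer is an empty stub.
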(event OnComponentBeginOverlap(ZoomCollision)
  (params (OverlappedComponent :type Primitive%20Component%20Object%20Reference) (OtherActor :type Actor%20Object%20Reference) (OtherComp :type Primitive%20Component%20Object%20Reference) (OtherBodyIndex :type Integer) (bFromSweep :type Boolean) (SweepResult :type Hit%20Result%20Structure%20%28by%20ref%29))
  ;[1 1 1] ZoomIn을 하기 위한 오버랩 이벤트
  (CallFunction|BeginOverlapPuzzle OtherActor self (Variables|Default|GetCamera)))

(event OnComponentEndOverlap(ZoomCollision)
  (params (OverlappedComponent :type Primitive%20Component%20Object%20Reference) (OtherActor :type Actor%20Object%20Reference) (OtherComp :type Primitive%20Component%20Object%20Reference) (OtherBodyIndex :type Integer))
  ;[1 1 1] ZoomIn을 하기 위한 오버랩 이벤트
  (CallFunction|EndOverlapPuzzle OtherActor))

(event OnComponentBeginOverlap(ArrowCollision1)
  (params (OverlappedComponent :type Primitive%20Component%20Object%20Reference) (OtherActor :type Actor%20Object%20Reference) (OtherComp :type Primitive%20Component%20Object%20Reference) (OtherBodyIndex :type Integer) (bFromSweep :type Boolean) (SweepResult :type Hit%20Result%20Structure%20%28by%20ref%29))
  ;[1 1 1] 화살표가 가리키는 부분 컴포넌트 가져오기
  (bind _as스태틱_메시_컴포넌트 (Utilities|Casting|CastToStaticMeshComponent OtherComp))
  (Variables|Default|SetSelected1 _as스태틱_메시_컴포넌트))

(event OnComponentBeginOverlap(ArrowCollision2)
  (params (OverlappedComponent :type Primitive%20Component%20Object%20Reference) (OtherActor :type Actor%20Object%20Reference) (OtherComp :type Primitive%20Component%20Object%20Reference) (OtherBodyIndex :type Integer) (bFromSweep :type Boolean) (SweepResult :type Hit%20Result%20Structure%20%28by%20ref%29))
  ;[1 1 1] 화살표가 가리키는 부분 컴포넌트 가져오기
  (bind _as스태틱_메시_컴포넌트 (Utilities|Casting|CastToStaticMeshComponent OtherComp))
  (Variables|Default|SetSelected2 _as스태틱_메시_컴포넌트))

(event Custom|CheckAnswer
  ;[1 1 1] 정답확인
)

(event Custom|CheckDoPuzzle
  ;[1 1 1] 퍼즐을 푸는 중인지 확인
  (bind _asbp_first_person_character (Utilities|Casting|CastToBP_FirstPersonCharacter (Game|GetPlayerCharacter 0)))
  (if (== (Variables|/Game/FirstPerson/Blueprints/BP_FirstPersonCharacter.BP_FirstPersonCharacter_C|GetBP_Puzzles _asbp_first_person_character) self)
    (Variables|Default|SetdoPuzzle (Variables|/Game/FirstPerson/Blueprints/BP_FirstPersonCharacter.BP_FirstPersonCharacter_C|GetCameraExpanded? _asbp_first_person_character))))

(event Custom|SwitchMaterial
  (params (Target :type Static%20Mesh%20Component%20Object%20Reference))
  (bind _returnvalue (Rendering|Material|GetMaterial Target 0))
  (bind _returnvalue_2 (Utilities|GetObjectName _returnvalue))
  ;[1 1 1] 머티리얼 스위칭
  (if (Utilities|Enum|Equal(Enum) _returnvalue_2 (Variables|Default|GetonMaterial))
    (Rendering|Material|SetMaterial Target 0 "/Game/Evidence+Puzzle_Asset/DoorPuzzle2_1/MM_DoorPuzzle2_1_Off.MM_DoorPuzzle2_1_Off")
    (elif (Utilities|Enum|Equal(Enum) _returnvalue_2 (Variables|Default|GetoffMaterial))
      (Rendering|Material|SetMaterial Target 0 "/Game/Evidence+Puzzle_Asset/DoorPuzzle2_1/MM_DoorPuzzle2_1_On.MM_DoorPuzzle2_1_On"))))

(event EventBeginPlay
  ;[1 1 1] 마우스이벤트를 받을 수 있도록 설정
  (Input|EnableInput (Game|GetPlayerController 0))
  ;[1 1 1] 초기값 설정
  (Variables|Default|SetSelected1 (Variables|Default|GetCircularPart5))
  (Variables|Default|SetSelected2 (Variables|Default|GetCircularPart6)))

(event Input|MouseEvents|LeftMouseButton
  (params (Key :type Key%20Structure :default "None"))
  ;[1 1 1] 클릭시 머티리얼 변경
  (:Pressed
    (CallFunction|CheckDoPuzzle)
    (if (Variables|Default|GetdoPuzzle)
      (CallFunction|SwitchMaterial (Variables|Default|GetSelected1))
      (CallFunction|SwitchMaterial (Variables|Default|GetSelected2)))))

(event Input|KeyboardEvents|D
  (params (Key :type Key%20Structure :default "None"))
  ;[1 1 1] 화살표 회전 이벤트
  (:Pressed
    (CallFunction|CheckDoPuzzle)
    (if (Variables|Default|GetdoPuzzle)
      (if (not (Variables|Default|GetisClicked))
        (bind _rotateclockwisevalue (Timeline|RotateClockwise PlayFromStart)
          (:Update
            (Variables|Default|SetisClicked true)
            (Transformation|SetWorldRotation (Variables|Default|GetMainButton) (Math|Rotator|MakeRotator 0.0 0.0 (+ _rotateclockwisevalue (Variables|Default|GetrotationZ))) false false))
          (:Finished
            (Variables|Default|SetrotationZ (+ _rotateclockwisevalue (Variables|Default|GetrotationZ)))
            (Variables|Default|SetisClicked false)))))))

(event Input|KeyboardEvents|A
  (params (Key :type Key%20Structure :default "None"))
  ;[1 1 1] 화살표 회전 이벤트
  (:Pressed
    (CallFunction|CheckDoPuzzle)
    (if (Variables|Default|GetdoPuzzle)
      (if (not (Variables|Default|GetisClicked))
        (bind _rotateclockwisevalue (Timeline|RotateCounterClockwise PlayFromStart)
          (:Update
            (Variables|Default|SetisClicked true)
            (Transformation|SetWorldRotation (Variables|Default|GetMainButton) (Math|Rotator|MakeRotator 0.0 0.0 (- (Variables|Default|GetrotationZ) _rotateclockwisevalue)) false false))
          (:Finished
            (Variables|Default|SetrotationZ (- (Variables|Default|GetrotationZ) _rotateclockwisevalue))
            (Variables|Default|SetisClicked false)))))))

(fn ConstructionScript)