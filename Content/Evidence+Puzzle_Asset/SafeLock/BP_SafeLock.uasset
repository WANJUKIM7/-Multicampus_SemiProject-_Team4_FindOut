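; BP_SafeLock is a safe prop in the evidence and puzzle assets that swings its rotation pivot open when triggered.
; The Trigger event eases RotationPivot to a fixed yaw over one second, with no combination or lock check in this Blueprint.
; BeginPlay enables input for the first player controller, labeled as an input test.
; Collision setup for SafeDoor and SafeMain is present but disconnected, so it never runs.
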(event EventBeginPlay
  ;[1 1 1] Input Test
  (Input|EnableInput (Game|GetPlayerController 0)))

(event EventTrigger
  (bind _rotationpivot (Variables|Default|GetRotationPivot))
  (bind _relativerotation (Variables|/Script/Engine.SceneComponent|GetRelativeRotation _rotationpivot))
  ;[1 1 1] Trigger Event
  (Components|MoveComponentTo _rotationpivot (Variables|/Script/Engine.SceneComponent|GetRelativeLocation _rotationpivot) (Math|Rotator|MakeRotator (.roll _relativerotation) (.pitch _relativerotation) -8e+01) true true 1.0 false))

(fn ConstructionScript)