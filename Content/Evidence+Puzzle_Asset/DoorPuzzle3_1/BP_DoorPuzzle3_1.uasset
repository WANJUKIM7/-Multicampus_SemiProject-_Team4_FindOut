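; Door circuit puzzle in which the player selects one of four circuit buttons with A/D and rotates its circuit with Space.
; ZoomCollision overlaps begin and end the puzzle interaction; input works only while the character's camera is expanded on this puzzle.
; The selected button gets a custom-depth highlight and brighter circuit.
; SetMaterial, mirrored in the construction script, pushes rotation and light values into material parameters; no solve check is present.
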(event OnComponentBeginOverlap(ZoomCollision)
  (params (OverlappedComponent :type Primitive%20Component%20Object%20Reference) (OtherActor :type Actor%20Object%20Reference) (OtherComp :type Primitive%20Component%20Object%20Reference) (OtherBodyIndex :type Integer) (bFromSweep :type Boolean) (SweepResult :type Hit%20Result%20Structure%20%28by%20ref%29))
  ;[1 1 1] ZoomIn을 하기 위한 오버랩 이벤트
  (CallFunction|BeginOverlapPuzzle OtherActor self (Variables|Default|GetCamera)))

(event OnComponentEndOverlap(ZoomCollision)
  (params (OverlappedComponent :type Primitive%20Component%20Object%20Reference) (OtherActor :type Actor%20Object%20Reference) (OtherComp :type Primitive%20Component%20Object%20Reference) (OtherBodyIndex :type Integer))
  ;[1 1 1] ZoomIn을 하기 위한 오버랩 이벤트
  (CallFunction|EndOverlapPuzzle))

(event Custom|SetLight
  (params (LightValue :type Float%20%28double-precision%29))
  ;[1 1 1] 밝기
  (switch int (Variables|Default|GetButtonIdx)
    (:0
      (Variables|Default|SetCircuitLight01 LightValue))
    (:1
      (Variables|Default|SetCircuitLight02 LightValue))
    (:2
      (Variables|Default|SetCircuitLight03 LightValue))
    (:3
      (Variables|Default|SetCircuitLight04 LightValue))))

(event Custom|InitHighlight
  ;[1 1 1] 퍼즐에 진입시
  (Rendering|SetRenderCustomDepth (Variables|Default|GetCurButton) true)
  (CallFunction|SetLight 1.0)
  (CallFunction|SetMaterial))

(event Custom|EndHighlight
  ;[1 1 1] 퍼즐에서 나올 시
  (Rendering|SetRenderCustomDepth (Variables|Default|GetCurButton) false))

(event Custom|SetCurrentButton
  ;[1 1 1] 버튼 설정
  (switch int (Variables|Default|GetButtonIdx)
    (:0
      (Variables|Default|SetCurButton (Variables|Default|GetCircuit_Button01_Door3_1)))
    (:1
      (Variables|Default|SetCurButton (Variables|Default|GetCircuit_Button02_Door3_1)))
    (:2
      (Variables|Default|SetCurButton (Variables|Default|GetCircuit_Button03_Door3_1)))
    (:3
      (Variables|Default|SetCurButton (Variables|Default|GetCircuit_Button04_Door3_1)))))

(event Custom|SetCircuitRotation
  ;[1 1 1] 회로버튼 회전
  (switch int (Variables|Default|GetButtonIdx)
    (:0
      (if (== (+ (Variables|Default|GetCircuitRotation01) (Variables|Default|Getgap)) 1.0)
        (Variables|Default|SetCircuitRotation01 0.0)
        (else
          (Variables|Default|SetCircuitRotation01 (+ (Variables|Default|GetCircuitRotation01) (Variables|Default|Getgap))))))
    (:1
      (if (== (+ (Variables|Default|GetCircuitRotation02) (Variables|Default|Getgap)) 1.0)
        (Variables|Default|SetCircuitRotation02 0.0)
        (else
          (Variables|Default|SetCircuitRotation02 (+ (Variables|Default|GetCircuitRotation02) (Variables|Default|Getgap))))))
    (:2
      (if (== (+ (Variables|Default|GetCircuitRotation03) (Variables|Default|Getgap)) 1.0)
        (Variables|Default|SetCircuitRotation03 0.0)
        (else
          (Variables|Default|SetCircuitRotation03 (+ (Variables|Default|GetCircuitRotation03) (Variables|Default|Getgap))))))
    (:3
      (if (== (+ (Variables|Default|GetCircuitRotation04) (Variables|Default|Getgap)) 1.0)
        (Variables|Default|SetCircuitRotation04 0.0)
        (else
          (Variables|Default|SetCircuitRotation04 (+ (Variables|Default|GetCircuitRotation04) (Variables|Default|Getgap))))))))

(event Custom|CheckDoPuzzle
  ;[1 1 1] 퍼즐을 푸는 중인지 확인
  (bind _asbp_first_person_character (Utilities|Casting|CastToBP_FirstPersonCharacter (Game|GetPlayerCharacter 0)))
  (if (== (Variables|/Game/FirstPerson/Blueprints/BP_FirstPersonCharacter.BP_FirstPersonCharacter_C|GetBP_Puzzles _asbp_first_person_character) self)
    (Variables|Default|SetdoPuzzle (Variables|/Game/FirstPerson/Blueprints/BP_FirstPersonCharacter.BP_FirstPersonCharacter_C|GetCameraExpanded? _asbp_first_person_character))))

(event EventBeginPlay
  ;[1 1 1] 초기값설정
  (Variables|Default|SetCurButton (Variables|Default|GetCircuit_Button01_Door3_1)))

(event Input|KeyboardEvents|A
  (params (Key :type Key%20Structure))
  ;[1 1 1] 버튼간 이동
  (:Pressed
    (CallFunction|CheckDoPuzzle)
    (if (Variables|Default|GetdoPuzzle)
      (Rendering|SetRenderCustomDepth (Variables|Default|GetcurButton) false)
      (CallFunction|SetLight 0.3)
      (Variables|Default|SetButtonIdx (Math|Integer|Clamp(Integer) (- (Variables|Default|GetButtonIdx) 1) 0 3))
      (CallFunction|SetCurrentButton)
      (Rendering|SetRenderCustomDepth (Variables|Default|GetcurButton) true)
      (CallFunction|SetLight 1.0)
      (CallFunction|SetMaterial))))

(event Input|KeyboardEvents|D
  (params (Key :type Key%20Structure))
  ;[1 1 1] 버튼간 이동
  (:Pressed
    (CallFunction|CheckDoPuzzle)
    (if (Variables|Default|GetdoPuzzle)
      (Rendering|SetRenderCustomDepth (Variables|Default|GetcurButton) false)
      (CallFunction|SetLight 0.3)
      (Variables|Default|SetButtonIdx (Math|Integer|Clamp(Integer) (+ (Variables|Default|GetButtonIdx) 1) 0 3))
      (CallFunction|SetCurrentButton)
      (Rendering|SetRenderCustomDepth (Variables|Default|GetcurButton) true)
      (CallFunction|SetLight 1.0)
      (CallFunction|SetMaterial))))

(event Input|KeyboardEvents|SpaceBar
  (params (Key :type Key%20Structure))
  ;[1 1 1] 버튼간 이동
  (:Pressed
    (CallFunction|CheckDoPuzzle)
    (if (Variables|Default|GetdoPuzzle)
      (CallFunction|SetCircuitRotation)
      (CallFunction|SetMaterial))))

(fn ConstructionScript
  (Utilities|FlowControl|Sequence
    (:then_0
      ;[1 1 1] 회로에 회전값 변수 설정
      (Rendering|Material|SetScalarParameterValueonMaterials (Variables|Default|GetCircuit01_South) "Rotation" (- 1.0 (Variables|Default|GetCircuitRotation01)))
      (Rendering|Material|SetScalarParameterValueonMaterials (Variables|Default|GetCircuit02_North) "Rotation" (- 1.0 (Variables|Default|GetCircuitRotation02)))
      (Rendering|Material|SetScalarParameterValueonMaterials (Variables|Default|GetCircuit03_South) "Rotation" (- 1.0 (Variables|Default|GetCircuitRotation03)))
      (Rendering|Material|SetScalarParameterValueonMaterials (Variables|Default|GetCircuit04_South) "Rotation" (- 1.0 (Variables|Default|GetCircuitRotation04)))
      ;[1 1 1] 밝기 조절
      (Rendering|Material|SetScalarParameterValueonMaterials (Variables|Default|GetCircuit01_South) "On=1,,,Off=0" (Variables|Default|GetCircuitLight01))
      (Rendering|Material|SetScalarParameterValueonMaterials (Variables|Default|GetCircuit02_North) "On=1,,,Off=0" (Variables|Default|GetCircuitLight02))
      (Rendering|Material|SetScalarParameterValueonMaterials (Variables|Default|GetCircuit03_South) "On=1,,,Off=0" (Variables|Default|GetCircuitLight03))
      (Rendering|Material|SetScalarParameterValueonMaterials (Variables|Default|GetCircuit04_South) "On=1,,,Off=0" (Variables|Default|GetCircuitLight04)))
    (:then_1
      ;[1 1 1] 와이어 파워 밝기조절
      (Rendering|Material|SetScalarParameterValueonMaterials (Variables|Default|GetWire01) "On=1,,,Off=0" (Variables|Default|GetWireLight))
      (Rendering|Material|SetScalarParameterValueonMaterials (Variables|Default|GetReceive02) "PowerOn=1,,,Off=0" (Variables|Default|GetPowerLight)))))

(fn SetMaterial
  (Utilities|FlowControl|Sequence
    (:then_0
      ;[1 1 1] 회로에 회전값 변수 설정
      (Rendering|Material|SetScalarParameterValueonMaterials (Variables|Default|GetCircuit01_South) "Rotation" (- 1.0 (Variables|Default|GetCircuitRotation01)))
      (Rendering|Material|SetScalarParameterValueonMaterials (Variables|Default|GetCircuit02_North) "Rotation" (- 1.0 (Variables|Default|GetCircuitRotation02)))
      (Rendering|Material|SetScalarParameterValueonMaterials (Variables|Default|GetCircuit03_South) "Rotation" (- 1.0 (Variables|Default|GetCircuitRotation03)))
      (Rendering|Material|SetScalarParameterValueonMaterials (Variables|Default|GetCircuit04_South) "Rotation" (- 1.0 (Variables|Default|GetCircuitRotation04)))
      ;[1 1 1] 밝기 조절
      (Rendering|Material|SetScalarParameterValueonMaterials (Variables|Default|GetCircuit01_South) "On=1,,,Off=0" (Variables|Default|GetCircuitLight01))
      (Rendering|Material|SetScalarParameterValueonMaterials (Variables|Default|GetCircuit02_North) "On=1,,,Off=0" (Variables|Default|GetCircuitLight02))
      (Rendering|Material|SetScalarParameterValueonMaterials (Variables|Default|GetCircuit03_South) "On=1,,,Off=0" (Variables|Default|GetCircuitLight03))
      (Rendering|Material|SetScalarParameterValueonMaterials (Variables|Default|GetCircuit04_South) "On=1,,,Off=0" (Variables|Default|GetCircuitLight04)))
    (:then_1
      ;[1 1 1] 와이어 파워 밝기조절
      (Rendering|Material|SetScalarParameterValueonMaterials (Variables|Default|GetWire01) "On=1,,,Off=0" (Variables|Default|GetWireLight))
      (Rendering|Material|SetScalarParameterValueonMaterials (Variables|Default|GetReceive02) "PowerOn=1,,,Off=0" (Variables|Default|GetPowerLight)))))