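; BP_CircuitPuzzle is an actor for a circuit puzzle, setting the visual rotation of three circuits, each built from North, South, East and West components.
; The Construction Script passes one minus each circuit's rotation variable to the "Rotation" scalar material parameter on that circuit's four components.
; Rotation is thus driven through materials at construction time, and the event graph holds no runtime logic.
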(event Collision|EventActorBeginOverlap
  (params (OtherActor :type Actor%20Object%20Reference)))

(event EventTick
  (params (DeltaSeconds :type Float%20%28single-precision%29)))

(event EventBeginPlay)

(fn ConstructionScript
  ;[1 1 1] 회로에 회전값 변수 설정
  (Rendering|Material|SetScalarParameterValueonMaterials (Variables|Default|GetCircuit01_South) "Rotation" (- 1.0 (Variables|Default|Get1_1Circuit01Rotation)))
  (Rendering|Material|SetScalarParameterValueonMaterials (Variables|Default|GetCircuit02_North) "Rotation" (- 1.0 (Variables|Default|Get1_1Circuit02Rotation)))
  (Rendering|Material|SetScalarParameterValueonMaterials (Variables|Default|GetCircuit03_North) "Rotation" (- 1.0 (Variables|Default|Get1_1Circuit03Rotation))))