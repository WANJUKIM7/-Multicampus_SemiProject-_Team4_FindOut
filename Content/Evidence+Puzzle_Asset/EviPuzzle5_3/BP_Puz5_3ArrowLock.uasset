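; Directional arrow padlock puzzle that the player solves while the camera is zoomed in on it.
; Zoom collision overlaps register the puzzle, and CheckDoPuzzle gates keys on the character's current puzzle, zoom state and IsClear.
; WASD timelines slide the cylinder and append directions to InputList, Space clears it, and X compares it to AnswerList.
; Timelines animate the lock head on success or failure, with success setting IsClear.
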(event OnComponentBeginOverlap(ZoomCollision)
  (params (OverlappedComponent :type Primitive%20Component%20Object%20Reference) (OtherActor :type Actor%20Object%20Reference) (OtherComp :type Primitive%20Component%20Object%20Reference) (OtherBodyIndex :type Integer) (bFromSweep :type Boolean) (SweepResult :type Hit%20Result%20Structure%20%28by%20ref%29))
  ;[1 1 1] ZoomIn을 하기 위한 오버랩 이벤트
  (CallFunction|BeginOverlapPuzzle OtherActor self (Variables|Default|GetCamera)))

(event OnComponentEndOverlap(ZoomCollision)
  (params (OverlappedComponent :type Primitive%20Component%20Object%20Reference) (OtherActor :type Actor%20Object%20Reference) (OtherComp :type Primitive%20Component%20Object%20Reference) (OtherBodyIndex :type Integer))
  ;[1 1 1] ZoomIn을 하기 위한 오버랩 이벤트
  (CallFunction|EndOverlapPuzzle))

(event Custom|CheckAnswer
  ;[1 1 1] 정답확인
  (if (== (Utilities|Array|Length (Variables|Default|GetinputList)) (Utilities|Array|Length (Variables|Default|GetAnswerList)))
    (Variables|Default|SetisSuccess true)
    (bind (_array_element _array_index) (Utilities|Array|ForEachLoopwithBreak (Variables|Default|GetAnswerList))
      (:LoopBody
        (if (not (Utilities|Enum|Equal(Enum) _array_element (Utilities|Array|Get(acopy) (Variables|Default|GetinputList) _array_index)))
          (Variables|Default|SetisSuccess false)
          (CallFunction|NotEqual)))
      (:Completed
        (if (Variables|Default|GetisSuccess)
          (CallFunction|Success)
          (else
            (CallFunction|Fail :!label _label)))))
    (else
      (goto _label))))

(event Custom|NotEqual
  ;[1 1 1] 정답확인
  (Utilities|Array|ForEachLoopwithBreak (Variables|Default|GetAnswerList)) ; enters at Break
)

(event Custom|Success
  ;[1 1 1] 성공
  (CallFunction|CheckDoPuzzle)
  (if (Variables|Default|GetdoPuzzle)
    (if (not (Variables|Default|GetisMoving))
      (bind _movelength (Timeline|TL_Success PlayFromStart)
        (:Update
          (Variables|Default|SetisMoving true)
          (bind _output_get (Variables|Default|SetmoveValue _movelength))
          (Transformation|SetRelativeLocation (Variables|Default|GetPuz5_3ArrowLockHead) (Math|Vector|MakeVector 0.0 0.0 _output_get) false false)
          (Variables|Default|SetisClear true))
        (:Finished
          (Variables|Default|SetisMoving false))))))

(event Custom|Fail
  ;[1 1 1] 실패
  (CallFunction|CheckDoPuzzle)
  (if (Variables|Default|GetdoPuzzle)
    (if (not (Variables|Default|GetisMoving))
      (bind _movelength (Timeline|TL_Fail PlayFromStart)
        (:Update
          (Variables|Default|SetisMoving true)
          (bind _output_get (Variables|Default|SetmoveValue _movelength))
          (Transformation|SetRelativeLocation (Variables|Default|GetPuz5_3ArrowLockHead) (Math|Vector|MakeVector 0.0 0.0 _output_get) false false))
        (:Finished
          (Variables|Default|SetisMoving false))))))

(event Custom|CheckDoPuzzle
  ;[1 1 1] 퍼즐을 푸는 중인지 확인
  (bind _asbp_first_person_character (Utilities|Casting|CastToBP_FirstPersonCharacter (Game|GetPlayerCharacter 0)))
  (if (== (Variables|/Game/FirstPerson/Blueprints/BP_FirstPersonCharacter.BP_FirstPersonCharacter_C|GetBP_Puzzles _asbp_first_person_character) self)
    (if (Variables|Default|GetisClear)
      (Variables|Default|SetdoPuzzle false)
      (else
        (Variables|Default|SetdoPuzzle (Variables|/Game/FirstPerson/Blueprints/BP_FirstPersonCharacter.BP_FirstPersonCharacter_C|GetCameraZoomed? _asbp_first_person_character))))))

(event EventBeginPlay
  ;[1 1 1] 초기값설정
)

(event EventZoomonEvent
  (params (PlayerCharacter :type BP%20First%20Person%20Character%20Object%20Reference))
  ;[1 1 1] 퍼즐에 진입시
)

(event EventZoomOutEvent
  ;[1 1 1] 퍼즐에서 나올 시
)

(event Input|KeyboardEvents|W
  (params (Key :type Key%20Structure :default "None"))
  ;[1 1 1] 버튼이동
  (:Pressed
    (CallFunction|CheckDoPuzzle)
    (if (Variables|Default|GetdoPuzzle)
      (if (not (Variables|Default|GetisMoving))
        (bind _output_get (Variables|Default|SetbuttonDir "NewEnumerator0"))
        (bind _movelength (Timeline|TL_MoveUp PlayFromStart)
          (:Update
            (Variables|Default|SetisMoving true)
            (bind _output_get_2 (Variables|Default|SetmoveValue _movelength))
            (Transformation|SetRelativeLocation (Variables|Default|GetPuz5_3ArrowLockCylinder) (Math|Vector|MakeVector 0.0 0.0 _output_get_2) false false))
          (:Finished
            (Utilities|Array|Add (Variables|Default|GetinputList) _output_get)
            (Variables|Default|SetisMoving false)))))))

(event Input|KeyboardEvents|S
  (params (Key :type Key%20Structure :default "None"))
  ;[1 1 1] 버튼이동
  (:Pressed
    (CallFunction|CheckDoPuzzle)
    (if (Variables|Default|GetdoPuzzle)
      (if (not (Variables|Default|GetisMoving))
        (bind _output_get (Variables|Default|SetbuttonDir "NewEnumerator1"))
        (bind _movelength (Timeline|TL_MoveDown PlayFromStart)
          (:Update
            (Variables|Default|SetisMoving true)
            (bind _output_get_2 (Variables|Default|SetmoveValue _movelength))
            (Transformation|SetRelativeLocation (Variables|Default|GetPuz5_3ArrowLockCylinder) (Math|Vector|MakeVector 0.0 0.0 (* _output_get_2 -1.0)) false false))
          (:Finished
            (Utilities|Array|Add (Variables|Default|GetinputList) _output_get)
            (Variables|Default|SetisMoving false)))))))

(event Input|KeyboardEvents|A
  (params (Key :type Key%20Structure :default "None"))
  ;[1 1 1] 버튼이동
  (:Pressed
    (CallFunction|CheckDoPuzzle)
    (if (Variables|Default|GetdoPuzzle)
      (if (not (Variables|Default|GetisMoving))
        (bind _output_get (Variables|Default|SetbuttonDir "NewEnumerator2"))
        (bind _movelength (Timeline|TL_MoveLeft PlayFromStart)
          (:Update
            (Variables|Default|SetisMoving true)
            (bind _output_get_2 (Variables|Default|SetmoveValue _movelength))
            (Transformation|SetRelativeLocation (Variables|Default|GetPuz5_3ArrowLockCylinder) (Math|Vector|MakeVector (* _output_get_2 -1.0) 0.0 0.0) false false))
          (:Finished
            (Utilities|Array|Add (Variables|Default|GetinputList) _output_get)
            (Variables|Default|SetisMoving false)))))))

(event Input|KeyboardEvents|D
  (params (Key :type Key%20Structure :default "None"))
  ;[1 1 1] 버튼이동
  (:Pressed
    (CallFunction|CheckDoPuzzle)
    (if (Variables|Default|GetdoPuzzle)
      (if (not (Variables|Default|GetisMoving))
        (bind _output_get (Variables|Default|SetbuttonDir "NewEnumerator3"))
        (bind _movelength (Timeline|TL_MoveRight PlayFromStart)
          (:Update
            (Variables|Default|SetisMoving true)
            (bind _output_get_2 (Variables|Default|SetmoveValue _movelength))
            (Transformation|SetRelativeLocation (Variables|Default|GetPuz5_3ArrowLockCylinder) (Math|Vector|MakeVector _output_get_2 0.0 0.0) false false))
          (:Finished
            (Utilities|Array|Add (Variables|Default|GetinputList) _output_get)
            (Variables|Default|SetisMoving false)))))))

(event Input|KeyboardEvents|SpaceBar
  (params (Key :type Key%20Structure :default "None"))
  ;[1 1 1] 버튼이동
  (:Pressed
    (CallFunction|CheckDoPuzzle)
    (if (Variables|Default|GetdoPuzzle)
      (if (not (Variables|Default|GetisMoving))
        (bind _movelength (Timeline|TL_ClearInput PlayFromStart)
          (:Update
            (Variables|Default|SetisMoving true)
            (bind _output_get (Variables|Default|SetmoveValue _movelength))
            (Transformation|SetRelativeLocation (Variables|Default|GetPuz5_3ArrowLockCylinder) (Math|Vector|MakeVector 0.0 (* _output_get -1.0) 0.0) false false))
          (:Finished
            (Utilities|Array|Clear (Variables|Default|GetinputList))
            (Variables|Default|SetisMoving false)))))))

(event Input|KeyboardEvents|X
  (params (Key :type Key%20Structure :default "None"))
  ;[1 1 1] 버튼이동
  (:Pressed
    (CallFunction|CheckDoPuzzle)
    (if (Variables|Default|GetdoPuzzle)
      (if (not (Variables|Default|GetisMoving))
        (CallFunction|CheckAnswer)))))

(fn ConstructionScript)