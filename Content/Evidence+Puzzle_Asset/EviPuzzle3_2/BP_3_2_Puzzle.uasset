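; Safe-lock puzzle Blueprint where seven sliding cylinder buttons must match an answer list to open a safe.
; Overlapping the zoom collision registers the puzzle, and zooming in highlights the current button through custom depth.
; While zoomed and unsolved, W/S select a button, A/D slide it between clamped positions stored in InputList, and X checks the answer.
; A match marks it solved and swings RotationPivot open with sound; failure has no effect.
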(event OnComponentBeginOverlap(ZoomCollision)
  (params (OverlappedComponent :type Primitive%20Component%20Object%20Reference) (OtherActor :type Actor%20Object%20Reference) (OtherComp :type Primitive%20Component%20Object%20Reference) (OtherBodyIndex :type Integer) (bFromSweep :type Boolean) (SweepResult :type Hit%20Result%20Structure%20%28by%20ref%29))
  ;[1 1 1] ZoomIn을 하기 위한 오버랩 이벤트
  (CallFunction|BeginOverlapPuzzle OtherActor self (Variables|Default|GetCamera)))

(event OnComponentEndOverlap(ZoomCollision)
  (params (OverlappedComponent :type Primitive%20Component%20Object%20Reference) (OtherActor :type Actor%20Object%20Reference) (OtherComp :type Primitive%20Component%20Object%20Reference) (OtherBodyIndex :type Integer))
  ;[1 1 1] ZoomIn을 하기 위한 오버랩 이벤트
  (CallFunction|EndOverlapPuzzle OtherActor))

(event Custom|CheckDoPuzzle
  ;[1 1 1] 퍼즐을 푸는 중인지 확인
  (bind _asbp_first_person_character (Utilities|Casting|CastToBP_FirstPersonCharacter (Game|GetPlayerCharacter 0)))
  (if (== (Variables|/Game/FirstPerson/Blueprints/BP_FirstPersonCharacter.BP_FirstPersonCharacter_C|GetBP_Puzzles _asbp_first_person_character) self)
    (if (Variables|Default|GetisClear)
      (Variables|Default|SetdoPuzzle false)
      (else
        (Variables|Default|SetdoPuzzle (Variables|/Game/FirstPerson/Blueprints/BP_FirstPersonCharacter.BP_FirstPersonCharacter_C|GetCameraZoomed? _asbp_first_person_character))))))

(event Custom|SetCurrentButton
  ;[1 1 1] 현재조작중인 버튼 설정
  (switch int (Variables|Default|GetcurButtonIdx)
    (:0
      (Variables|Default|SetcurButton (Variables|Default|Get3_2Cylinder1)))
    (:1
      (Variables|Default|SetcurButton (Variables|Default|Get3_2Cylinder2)))
    (:2
      (Variables|Default|SetcurButton (Variables|Default|Get3_2Cylinder3)))
    (:3
      (Variables|Default|SetcurButton (Variables|Default|Get3_2Cylinder4)))
    (:4
      (Variables|Default|SetcurButton (Variables|Default|Get3_2Cylinder5)))
    (:5
      (Variables|Default|SetcurButton (Variables|Default|Get3_2Cylinder6)))
    (:6
      (Variables|Default|SetcurButton (Variables|Default|Get3_2Cylinder7)))))

(event Custom|CheckAnswer
  ;[1 1 1] 정답확인
  (Variables|Default|SetisSuccess true)
  (bind (_array_element _array_index) (Utilities|Array|ForEachLoopwithBreak (Variables|Default|GetanswerList))
    (:LoopBody
      (if (not (== _array_element (Utilities|Array|Get(acopy) (Variables|Default|GetinputList) _array_index)))
        (Variables|Default|SetisSuccess false)
        (CallFunction|NotEqual)))
    (:Completed
      (if (Variables|Default|GetisSuccess)
        (CallFunction|Success)
        (else
          (CallFunction|Fail))))))

(event Custom|Open
  (bind _rotationpivot (Variables|Default|GetRotationPivot))
  (bind _relativerotation (Variables|/Script/Engine.SceneComponent|GetRelativeRotation _rotationpivot))
  ;[1 1 1] 금고 열기
  (Audio|PlaySound2D "/Game/Sounds_BGM+SE_/SoundEffects/SafeLockOpen.SafeLockOpen" 1.0 1.0 0.0 0 0)
  (Components|MoveComponentTo _rotationpivot (Variables|/Script/Engine.SceneComponent|GetRelativeLocation _rotationpivot) (Math|Rotator|MakeRotator (.roll _relativerotation) (.pitch _relativerotation) -9e+01) true true 3.0 false))

(event Custom|NotEqual
  ;[1 1 1] 정답확인
  (Utilities|Array|ForEachLoopwithBreak (Variables|Default|GetanswerList)) ; enters at Break
)

(event Custom|Success
  ;[1 1 1] 성공
  (CallFunction|CheckDoPuzzle)
  (if (Variables|Default|GetdoPuzzle)
    (if (not (Variables|Default|GetisMoving))
      (Rendering|SetRenderCustomDepth (Variables|Default|GetcurButton) false)
      (CallFunction|Open)
      (Variables|Default|SetisClear true)
      (Variables|Default|SetSolved? true))))

(event Custom|Fail
  ;[1 1 1] 실패
  (CallFunction|CheckDoPuzzle)
  (if (Variables|Default|GetdoPuzzle)
    _))

(event EventZoomonEvent
  (params (PlayerCharacter :type BP%20First%20Person%20Character%20Object%20Reference))
  ;[1 1 1] 퍼즐에 진입시 하이라이트 표시
  (|CallParentFunction PlayerCharacter)
  (if (not (Variables|Default|GetisClear))
    (Rendering|SetRenderCustomDepth (Variables|Default|GetcurButton) true)))

(event EventZoomOutEvent
  ;[1 1 1] 퍼즐에서 나올 시 하이라이트 표시 제거
  (|CallParentFunction)
  (Rendering|SetRenderCustomDepth (Variables|Default|GetcurButton) false))

(event EventBeginPlay
  ;[1 1 1] 초기값설정
  (Variables|Default|SetDisplayDescription "W,S to select button A,D to move button X to check answer")
  (Variables|Default|SetcurButton (Variables|Default|Get3_2Cylinder1)))

(event Input|KeyboardEvents|W
  (params (Key :type Key%20Structure :default "None"))
  ;[1 1 1] 키 입력에 따른 버튼 인덱스 설정 및 조작할 버튼 선택
  (:Pressed
    (CallFunction|CheckDoPuzzle)
    (if (Variables|Default|GetdoPuzzle)
      (Rendering|SetRenderCustomDepth (Variables|Default|GetcurButton) false)
      (Variables|Default|SetcurButtonIdx (Math|Integer|Clamp(Integer) (- (Variables|Default|GetcurButtonIdx) 1) 0 6))
      (CallFunction|SetCurrentButton)
      (Rendering|SetRenderCustomDepth (Variables|Default|GetcurButton) true)
      (Variables|Default|SetcurButtonValue (Utilities|Array|Get(acopy) (Variables|Default|GetinputList) (Variables|Default|GetcurButtonIdx)))
      (Audio|PlaySound2D "/Game/Sounds_BGM+SE_/SoundEffects/ClankSound__2_.ClankSound__2_" 1.0 1.0 0.0 0 0))))

(event Input|KeyboardEvents|S
  (params (Key :type Key%20Structure :default "None"))
  ;[1 1 1] 키 입력에 따른 버튼 인덱스 설정 및 조작할 버튼 선택
  (:Pressed
    (CallFunction|CheckDoPuzzle)
    (if (Variables|Default|GetdoPuzzle)
      (Rendering|SetRenderCustomDepth (Variables|Default|GetcurButton) false)
      (Variables|Default|SetcurButtonIdx (Math|Integer|Clamp(Integer) (+ (Variables|Default|GetcurButtonIdx) 1) 0 6))
      (CallFunction|SetCurrentButton)
      (Rendering|SetRenderCustomDepth (Variables|Default|GetcurButton) true)
      (Variables|Default|SetcurButtonValue (Utilities|Array|Get(acopy) (Variables|Default|GetinputList) (Variables|Default|GetcurButtonIdx)))
      (Audio|PlaySound2D "/Game/Sounds_BGM+SE_/SoundEffects/ClankSound__2_.ClankSound__2_" 1.0 1.0 0.0 0 0))))

(event Input|KeyboardEvents|A
  (params (Key :type Key%20Structure :default "None"))
  (bind _curbutton (Variables|Default|GetcurButton))
  ;[1 1 1] 키 입력에 따른 버튼 인덱스 설정 및 조작할 버튼 선택
  (:Pressed
    (CallFunction|CheckDoPuzzle)
    (if (Variables|Default|GetdoPuzzle)
      (bind _output_get (Variables|Default|SetnextButtonValue (Math|Integer|Clamp(Integer) (- (Variables|Default|GetcurButtonValue) 1) 1 7)))
      (if (!= _output_get (Variables|Default|GetcurButtonValue))
        (Transformation|SetWorldLocation _curbutton (- (Transformation|GetWorldLocation _curbutton) (Math|Vector|MakeVector (Variables|Default|Getgap) 0.0 0.0)) false false)
        (bind _output_get_2 (Variables|Default|SetcurButtonValue (Variables|Default|GetnextButtonValue)))
        (Utilities|Array|SetArrayElem (Variables|Default|GetinputList) (Variables|Default|GetcurButtonIdx) _output_get_2)
        (Audio|PlaySound2D "/Game/Sounds_BGM+SE_/SoundEffects/ClankSound__2_.ClankSound__2_" 1.0 1.0 0.0 0 0)))))

(event Input|KeyboardEvents|D
  (params (Key :type Key%20Structure :default "None"))
  (bind _curbutton (Variables|Default|GetcurButton))
  ;[1 1 1] 키 입력에 따른 버튼 인덱스 설정 및 조작할 버튼 선택
  (:Pressed
    (CallFunction|CheckDoPuzzle)
    (if (Variables|Default|GetdoPuzzle)
      (bind _output_get (Variables|Default|SetnextButtonValue (Math|Integer|Clamp(Integer) (+ (Variables|Default|GetcurButtonValue) 1) 1 7)))
      (if (!= _output_get (Variables|Default|GetcurButtonValue))
        (Transformation|SetWorldLocation _curbutton (+ (Transformation|GetWorldLocation _curbutton) (Math|Vector|MakeVector (Variables|Default|Getgap) 0.0 0.0)) false false)
        (bind _output_get_2 (Variables|Default|SetcurButtonValue (Variables|Default|GetnextButtonValue)))
        (Utilities|Array|SetArrayElem (Variables|Default|GetinputList) (Variables|Default|GetcurButtonIdx) _output_get_2)
        (Audio|PlaySound2D "/Game/Sounds_BGM+SE_/SoundEffects/ClankSound__2_.ClankSound__2_" 1.0 1.0 0.0 0 0)))))

(event Input|KeyboardEvents|X
  (params (Key :type Key%20Structure :default "None"))
  ;[1 1 1] 키 입력에 따른 버튼 인덱스 설정 및 조작할 버튼 선택
  (:Pressed
    (CallFunction|CheckDoPuzzle)
    (if (Variables|Default|GetdoPuzzle)
      (CallFunction|CheckAnswer))))

(fn ConstructionScript)