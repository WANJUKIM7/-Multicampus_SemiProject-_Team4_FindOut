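; Four-tumbler combination lock that unlocks its linked BPUnlockable when the tumbler digits match the Combination string.
; A delayed Tick compares the child-actor tumbler numbers about once a second, then runs a one-time sequence that briefly drops the lock mesh with physics and calls Unlock.
; Tumblers can randomize on BeginPlay.
; An overlap trigger, sized and placed by the construction script, toggles the first-person character's UsingLock flag.
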(event OnComponentBeginOverlap(LockTrigger)
  (params (OverlappedComponent :type Primitive%20Component%20Object%20Reference) (OtherActor :type Actor%20Object%20Reference) (OtherComp :type Primitive%20Component%20Object%20Reference) (OtherBodyIndex :type Integer) (bFromSweep :type Boolean) (SweepResult :type Hit%20Result%20Structure%20%28by%20ref%29))
  (bind _asbp_first_person_character (Utilities|Casting|CastToBP_FirstPersonCharacter OtherActor))
  (Variables|/Game/FirstPerson/Blueprints/BP_FirstPersonCharacter.BP_FirstPersonCharacter_C|SetUsingLock? _asbp_first_person_character true))

(event OnComponentEndOverlap(LockTrigger)
  (params (OverlappedComponent :type Primitive%20Component%20Object%20Reference) (OtherActor :type Actor%20Object%20Reference) (OtherComp :type Primitive%20Component%20Object%20Reference) (OtherBodyIndex :type Integer))
  (bind _asbp_first_person_character (Utilities|Casting|CastToBP_FirstPersonCharacter OtherActor))
  (Variables|/Game/FirstPerson/Blueprints/BP_FirstPersonCharacter.BP_FirstPersonCharacter_C|SetUsingLock? _asbp_first_person_character false))

(event EventTick
  (params (DeltaSeconds :type Float%20%28single-precision%29))
  ;[1 1 1] Check for Correct Combination
  (Utilities|FlowControl|Delay 1.0)
  (bind _combomatch_ (CallFunction|CheckCombination))
  (if _combomatch_
    (Utilities|FlowControl|DoOnce false
      (:Completed
        (Variables|Default|SetLockedState false)
        (Utilities|FlowControl|Delay 1.5)
        (Class|SkeletalMeshComponent|SetAllBodiesSimulatePhysics (Variables|Default|GetLockMesh) true)
        (Utilities|FlowControl|Delay 0.4)
        (Default|Unlock (Variables|LockSettings|GetBP_Unlockable))
        (Utilities|FlowControl|Delay 2.0)
        (Class|SkeletalMeshComponent|SetAllBodiesSimulatePhysics (Variables|Default|GetLockMesh) false)))))

(event EventBeginPlay
  ;[1 1 1] Randomize Tumblers?
  (if (Variables|LockSettings|GetRandomizeTumblerRotation?)
    (Default|RandomizeTumbler (.AsBP%20Lock%20Tumbler (Utilities|Casting|CastToBP_LockTumbler (Variables|/Script/Engine.ChildActorComponent|GetChildActor (Variables|Default|GetBP_LockTumbler1)))))
    (Default|RandomizeTumbler (.AsBP%20Lock%20Tumbler (Utilities|Casting|CastToBP_LockTumbler (Variables|/Script/Engine.ChildActorComponent|GetChildActor (Variables|Default|GetBP_LockTumbler2)))))
    (Default|RandomizeTumbler (.AsBP%20Lock%20Tumbler (Utilities|Casting|CastToBP_LockTumbler (Variables|/Script/Engine.ChildActorComponent|GetChildActor (Variables|Default|GetBP_LockTumbler3)))))
    (Default|RandomizeTumbler (.AsBP%20Lock%20Tumbler (Utilities|Casting|CastToBP_LockTumbler (Variables|/Script/Engine.ChildActorComponent|GetChildActor (Variables|Default|GetBP_LockTumbler4)))))))

(fn ConstructionScript
  (bind _locktrigger (Variables|Default|GetLockTrigger))
  (Transformation|SetRelativeScale3D _locktrigger (Variables|LockSettings|GetLockTriggerScale))
  (Transformation|SetRelativeLocation _locktrigger (Variables|LockSettings|GetLockTriggerLocation) false false))

(fn CheckCombination
  (return (Utilities|Enum|Equal(Enum) (Variables|LockSettings|GetCombination) (Utilities|String|Append (Utilities|String|ToString(Integer) (Variables|/Game/Blueprints/BP_LockTumbler.BP_LockTumbler_C|GetTumblerNumber (.AsBP%20Lock%20Tumbler (Utilities|Casting|CastToBP_LockTumbler (Variables|/Script/Engine.ChildActorComponent|GetChildActor (Variables|Default|GetBP_LockTumbler1)))))) (Utilities|String|ToString(Integer) (Variables|/Game/Blueprints/BP_LockTumbler.BP_LockTumbler_C|GetTumblerNumber (.AsBP%20Lock%20Tumbler (Utilities|Casting|CastToBP_LockTumbler (Variables|/Script/Engine.ChildActorComponent|GetChildActor (Variables|Default|GetBP_LockTumbler2)))))) (Utilities|String|ToString(Integer) (Variables|/Game/Blueprints/BP_LockTumbler.BP_LockTumbler_C|GetTumblerNumber (.AsBP%20Lock%20Tumbler (Utilities|Casting|CastToBP_LockTumbler (Variables|/Script/Engine.ChildActorComponent|GetChildActor (Variables|Default|GetBP_LockTumbler3)))))) (Utilities|String|ToString(Integer) (Variables|/Game/Blueprints/BP_LockTumbler.BP_LockTumbler_C|GetTumblerNumber (.AsBP%20Lock%20Tumbler (Utilities|Casting|CastToBP_LockTumbler (Variables|/Script/Engine.ChildActorComponent|GetChildActor (Variables|Default|GetBP_LockTumbler4))))))))))