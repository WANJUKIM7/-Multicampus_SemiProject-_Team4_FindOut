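; Interaction component that tracks the focused BP_interactionArea and toggles its focus state.
; Every tick, Trace compares the hit actor with the cached one and passes an exact class check to TraceInteractionArea, which switches or clears focus.
; The camera-forward visibility line trace is never executed, and nothing here sets the hit values that Trace reads.
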(event EventTick
  (params (DeltaSeconds :type Float%20%28single-precision%29))
  (CallFunction|Trace))

(fn Trace
  (bind _linetracehitactor (Variables|Default|GetLineTraceHitActor))
  (if (Variables|Default|GetLineTraceReturnValue)
    (if (!= (Variables|Default|GetFocusedActor) _linetracehitactor)
      (Variables|Default|SetFocusedActor _linetracehitactor)
      (CallFunction|TraceInteractionArea (== (Utilities|GetClass _linetracehitactor) "/Game/Programming/Outline/BP_interactionArea.BP_interactionArea_C")))
    (else
      (CallFunction|TraceInteractionArea false))))

(fn TraceInteractionArea
  (params (Trace :type Boolean))
  (if Trace
    (if (Variables|Default|GetIsTracingInteractionArea)
      (Default|ToggleFocus (Variables|Default|GetFocusedInteractionArea) false))
    (bind _asbp_interaction_area (Utilities|Casting|CastToBP_interactionArea (Variables|Default|GetFocusedActor)))
    (bind _output_get (Variables|Default|SetFocusedInteractionArea _asbp_interaction_area))
    (Default|ToggleFocus _output_get true)
    (Variables|Default|SetIsTracingInteractionArea true)
    (elif (Variables|Default|GetIsTracingInteractionArea)
      (Variables|Default|SetIsTracingInteractionArea false)
      (Default|ToggleFocus (Variables|Default|GetFocusedInteractionArea) false)
      (Variables|Default|SetFocusedActor 0)
      (Variables|Default|SetFocusedInteractionArea 0))))