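; Puzzle 3-1 actor with a zoom trigger volume, a Support piece and four Place pieces.
; Entering ZoomCollision passes the overlapping actor, the puzzle and its Camera to BeginOverlapPuzzle, and leaving calls EndOverlapPuzzle.
; Cursor-over events on the Support and Place pieces only print debug messages, and no puzzle-solving logic exists in these graphs.
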(event OnBeginCursorOver(Place1)
  (params (TouchedComponent :type Primitive%20Component%20Object%20Reference))
  (Development|PrintString "Puzzle_3_1 : Begin Cursor Over place1"))

(event OnComponentBeginOverlap(ZoomCollision)
  (params (OverlappedComponent :type Primitive%20Component%20Object%20Reference) (OtherActor :type Actor%20Object%20Reference) (OtherComp :type Primitive%20Component%20Object%20Reference) (OtherBodyIndex :type Integer) (bFromSweep :type Boolean) (SweepResult :type Hit%20Result%20Structure%20%28by%20ref%29))
  ;[1 1 1] 오버랩 이벤트
  (CallFunction|BeginOverlapPuzzle OtherActor self (Variables|Default|GetCamera)))

(event OnComponentEndOverlap(ZoomCollision)
  (params (OverlappedComponent :type Primitive%20Component%20Object%20Reference) (OtherActor :type Actor%20Object%20Reference) (OtherComp :type Primitive%20Component%20Object%20Reference) (OtherBodyIndex :type Integer))
  ;[1 1 1] 오버랩 이벤트
  (CallFunction|EndOverlapPuzzle))

(event OnBeginCursorOver(Place2)
  (params (TouchedComponent :type Primitive%20Component%20Object%20Reference))
  (Development|PrintString "Puzzle_3_1 : Begin Cursor Over place2"))

(event OnBeginCursorOver(Support)
  (params (TouchedComponent :type Primitive%20Component%20Object%20Reference))
  (Development|PrintString "Puzzle_3_1 : Begin Cursor Over Support"))

(event OnBeginCursorOver(Place3)
  (params (TouchedComponent :type Primitive%20Component%20Object%20Reference))
  (Development|PrintString "Puzzle_3_1 : Begin Cursor Over place3"))

(event OnBeginCursorOver(Place4)
  (params (TouchedComponent :type Primitive%20Component%20Object%20Reference))
  (Development|PrintString "Puzzle_3_1 : Begin Cursor Over place4"))

(fn ConstructionScript)