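; Four-tumbler combination lock puzzle with camera zoom, started through a trigger overlap.
; Cursor-over events bound on the child-actor tumblers select and custom-depth highlight one, and the mouse wheel spins it either way.
; After each spin, the joined tumbler digits are compared to Answer.
; A match disables input, briefly drops the lock with physics, zooms out, fires the linked Trigger and removes the overlap volume.
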(event OnComponentBeginOverlap(LockTrigger)
  (params (OverlappedComponent :type Primitive%20Component%20Object%20Reference) (OtherActor :type Actor%20Object%20Reference) (OtherComp :type Primitive%20Component%20Object%20Reference) (OtherBodyIndex :type Integer) (bFromSweep :type Boolean) (SweepResult :type Hit%20Result%20Structure%20%28by%20ref%29))
  ;[1 1 1] 카메라 줌 오버랩
  (CallFunction|BeginOverlapPuzzle OtherActor self (Variables|Default|GetCamera)))

(event OnComponentEndOverlap(LockTrigger)
  (params (OverlappedComponent :type Primitive%20Component%20Object%20Reference) (OtherActor :type Actor%20Object%20Reference) (OtherComp :type Primitive%20Component%20Object%20Reference) (OtherBodyIndex :type Integer))
  ;[1 1 1] 카메라 줌 오버랩
  (CallFunction|EndOverlapPuzzle OtherActor))

(event Custom|CheckAnswer
  ;[1 1 1] 번호 맞는지 확인
  (bind _combomatch_ (CallFunction|CheckCombination))
  (if _combomatch_
    (Input|DisableInput (Game|GetPlayerController 0))
    (Utilities|FlowControl|DoOnce false
      (:Completed
        (Variables|LockSettings|SetLockedState false)
        (Utilities|FlowControl|Delay 0.5)
        (Class|SkeletalMeshComponent|SetAllBodiesSimulatePhysics (Variables|Default|GetLockMesh) true)
        (CallFunction|ZoomOutPuzzle self)
        (Default|Trigger (Variables|Default|GetTrigger))
        (Variables|Default|SetTags (Variables|LockSettings|Get태그))
        (Utilities|FlowControl|Delay 0.4)
        (Utilities|FlowControl|Delay 2.0)
        (Class|SkeletalMeshComponent|SetAllBodiesSimulatePhysics (Variables|Default|GetLockMesh) false)
        (Components|DestroyComponent (Variables|Default|GetLockTrigger))))))

(event Custom|OnCursorOver1
  (params (TouchedActor :type Actor%20Object%20Reference))
  (bind _bp_locktumbler1 (Variables|Default|GetBP_LockTumbler1))
  (bind _childactor (Variables|/Script/Engine.ChildActorComponent|GetChildActor _bp_locktumbler1))
  (bind _asbp_lock_tumbler (Utilities|Casting|CastToBP_LockTumbler _childactor))
  ;[1 1 1] 시작시 이벤트 함수 설정.
  (Rendering|SetRenderCustomDepth (Variables|/Game/Programming/Blueprints/BP_LockTumbler.BP_LockTumbler_C|GetTumblerMesh _asbp_lock_tumbler) true)
  (Variables|LockSettings|SetSelectedTumbler _asbp_lock_tumbler))

(event Custom|EndCursorOver1
  (params (TouchedActor :type Actor%20Object%20Reference))
  ;[1 1 1] 시작시 이벤트 함수 설정.
  (Rendering|SetRenderCustomDepth (Variables|/Game/Programming/Blueprints/BP_LockTumbler.BP_LockTumbler_C|GetTumblerMesh (.AsBP%20Lock%20Tumbler (Utilities|Casting|CastToBP_LockTumbler (Variables|/Script/Engine.ChildActorComponent|GetChildActor (Variables|Default|GetBP_LockTumbler1))))) false)
  (Variables|LockSettings|SetSelectedTumbler 0))

(event Custom|OnCursorOver2
  (params (TouchedActor :type Actor%20Object%20Reference))
  (bind _bp_locktumbler2 (Variables|Default|GetBP_LockTumbler2))
  (bind _childactor (Variables|/Script/Engine.ChildActorComponent|GetChildActor _bp_locktumbler2))
  (bind _asbp_lock_tumbler (Utilities|Casting|CastToBP_LockTumbler _childactor))
  ;[1 1 1] 시작시 이벤트 함수 설정.
  (Rendering|SetRenderCustomDepth (Variables|/Game/Programming/Blueprints/BP_LockTumbler.BP_LockTumbler_C|GetTumblerMesh _asbp_lock_tumbler) true)
  (Variables|LockSettings|SetSelectedTumbler _asbp_lock_tumbler))

(event Custom|EndCursorOver2
  (params (TouchedActor :type Actor%20Object%20Reference))
  ;[1 1 1] 시작시 이벤트 함수 설정.
  (Rendering|SetRenderCustomDepth (Variables|/Game/Programming/Blueprints/BP_LockTumbler.BP_LockTumbler_C|GetTumblerMesh (.AsBP%20Lock%20Tumbler (Utilities|Casting|CastToBP_LockTumbler (Variables|/Script/Engine.ChildActorComponent|GetChildActor (Variables|Default|GetBP_LockTumbler2))))) false)
  (Variables|LockSettings|SetSelectedTumbler 0))

(event Custom|OnCursorOver3
  (params (TouchedActor :type Actor%20Object%20Reference))
  (bind _bp_locktumbler3 (Variables|Default|GetBP_LockTumbler3))
  (bind _childactor (Variables|/Script/Engine.ChildActorComponent|GetChildActor _bp_locktumbler3))
  (bind _asbp_lock_tumbler (Utilities|Casting|CastToBP_LockTumbler _childactor))
  ;[1 1 1] 시작시 이벤트 함수 설정.
  (Rendering|SetRenderCustomDepth (Variables|/Game/Programming/Blueprints/BP_LockTumbler.BP_LockTumbler_C|GetTumblerMesh _asbp_lock_tumbler) true)
  (Variables|LockSettings|SetSelectedTumbler _asbp_lock_tumbler))

(event Custom|EndCursorOver3
  (params (TouchedActor :type Actor%20Object%20Reference))
  ;[1 1 1] 시작시 이벤트 함수 설정.
  (Rendering|SetRenderCustomDepth (Variables|/Game/Programming/Blueprints/BP_LockTumbler.BP_LockTumbler_C|GetTumblerMesh (.AsBP%20Lock%20Tumbler (Utilities|Casting|CastToBP_LockTumbler (Variables|/Script/Engine.ChildActorComponent|GetChildActor (Variables|Default|GetBP_LockTumbler3))))) false)
  (Variables|LockSettings|SetSelectedTumbler 0))

(event Custom|OnCursorOver4
  (params (TouchedActor :type Actor%20Object%20Reference))
  (bind _bp_locktumbler4 (Variables|Default|GetBP_LockTumbler4))
  (bind _childactor (Variables|/Script/Engine.ChildActorComponent|GetChildActor _bp_locktumbler4))
  (bind _asbp_lock_tumbler (Utilities|Casting|CastToBP_LockTumbler _childactor))
  ;[1 1 1] 시작시 이벤트 함수 설정.
  (Rendering|SetRenderCustomDepth (Variables|/Game/Programming/Blueprints/BP_LockTumbler.BP_LockTumbler_C|GetTumblerMesh _asbp_lock_tumbler) true)
  (Variables|LockSettings|SetSelectedTumbler _asbp_lock_tumbler))

(event Custom|EndCursorOver4
  (params (TouchedActor :type Actor%20Object%20Reference))
  ;[1 1 1] 시작시 이벤트 함수 설정.
  (Rendering|SetRenderCustomDepth (Variables|/Game/Programming/Blueprints/BP_LockTumbler.BP_LockTumbler_C|GetTumblerMesh (.AsBP%20Lock%20Tumbler (Utilities|Casting|CastToBP_LockTumbler (Variables|/Script/Engine.ChildActorComponent|GetChildActor (Variables|Default|GetBP_LockTumbler4))))) false)
  (Variables|LockSettings|SetSelectedTumbler 0))

(event EventZoomonEvent
  (params (PlayerCharacter :type BP%20First%20Person%20Character%20Object%20Reference))
  ;[1 1 1] When Zoon On / Out
  (|CallParentFunction PlayerCharacter))

(event EventZoomOutEvent
  ;[1 1 1] When Zoon On / Out
  (|CallParentFunction)
  (CallFunction|EndCursorOver1)
  (CallFunction|EndCursorOver2)
  (CallFunction|EndCursorOver3)
  (CallFunction|EndCursorOver4))

(event EventBeginPlay
  (bind _bp_locktumbler1 (Variables|Default|GetBP_LockTumbler1))
  (bind _bp_locktumbler4 (Variables|Default|GetBP_LockTumbler4))
  (bind _bp_locktumbler3 (Variables|Default|GetBP_LockTumbler3))
  (bind _bp_locktumbler2 (Variables|Default|GetBP_LockTumbler2))
  (bind _childactor (Variables|/Script/Engine.ChildActorComponent|GetChildActor _bp_locktumbler1))
  (bind _childactor_2 (Variables|/Script/Engine.ChildActorComponent|GetChildActor _bp_locktumbler2))
  (bind _childactor_3 (Variables|/Script/Engine.ChildActorComponent|GetChildActor _bp_locktumbler3))
  (bind _childactor_4 (Variables|/Script/Engine.ChildActorComponent|GetChildActor _bp_locktumbler4))
  (bind _asbp_lock_tumbler (Utilities|Casting|CastToBP_LockTumbler _childactor_4))
  (bind _asbp_lock_tumbler_2 (Utilities|Casting|CastToBP_LockTumbler _childactor))
  (bind _asbp_lock_tumbler_3 (Utilities|Casting|CastToBP_LockTumbler _childactor_2))
  (bind _asbp_lock_tumbler_4 (Utilities|Casting|CastToBP_LockTumbler _childactor_3))
  ;[1 1 1] 시작시 이벤트 함수 설정.
  (Utilities|FlowControl|Sequence
    (:then_0
      (Variables|Default|SetDisplayDescription "Set the lock number using the mouse wheel"))
    (:then_1
      (EventDispatchers|BindEventtoOnBeginCursorOver _asbp_lock_tumbler_2 (delegate Custom|OnCursorOver1))
      (EventDispatchers|BindEventtoOnEndCursorOver _asbp_lock_tumbler_2 (delegate Custom|EndCursorOver1)))
    (:then_2
      (EventDispatchers|BindEventtoOnBeginCursorOver _asbp_lock_tumbler_3 (delegate Custom|OnCursorOver2))
      (EventDispatchers|BindEventtoOnEndCursorOver _asbp_lock_tumbler_3 (delegate Custom|EndCursorOver2)))
    (:then_3
      (EventDispatchers|BindEventtoOnBeginCursorOver _asbp_lock_tumbler_4 (delegate Custom|OnCursorOver3))
      (EventDispatchers|BindEventtoOnEndCursorOver _asbp_lock_tumbler_4 (delegate Custom|EndCursorOver3)))
    (:then_4
      (EventDispatchers|BindEventtoOnBeginCursorOver _asbp_lock_tumbler (delegate Custom|OnCursorOver4))
      (EventDispatchers|BindEventtoOnEndCursorOver _asbp_lock_tumbler (delegate Custom|EndCursorOver4)))))

(event Input|MouseEvents|MouseWheelUp
  (params (Key :type Key%20Structure :default "None"))
  ;[1 1 1] Spin Tumbler
  (:Pressed
    (if (not (Variables|LockSettings|GetRotating?))
      (Variables|LockSettings|SetRotating? true)
      (bind _selectedtumbler (Variables|LockSettings|GetSelectedTumbler)
        (:then
          (Default|SpinTumblerBackward _selectedtumbler)
          (Utilities|FlowControl|Delay 0.6)
          (CallFunction|CheckAnswer)
          (Variables|LockSettings|SetRotating? false))
        (:else)))))

(event Input|MouseEvents|MouseWheelDown
  (params (Key :type Key%20Structure :default "None"))
  ;[1 1 1] Spin Tumbler
  (:Pressed
    (if (not (Variables|LockSettings|GetRotating?))
      (Variables|LockSettings|SetRotating? true)
      (bind _selectedtumbler (Variables|LockSettings|GetSelectedTumbler)
        (:then
          (Default|SpinTumbler _selectedtumbler)
          (Utilities|FlowControl|Delay 0.6)
          (CallFunction|CheckAnswer)
          (Variables|LockSettings|SetRotating? false))
        (:else)))))

(fn ConstructionScript
  (bind _locktrigger (Variables|Default|GetLockTrigger))
  (Transformation|SetRelativeScale3D _locktrigger (Variables|LockSettings|GetLockTriggerScale))
  (Transformation|SetRelativeLocation _locktrigger (Variables|LockSettings|GetLockTriggerLocation) false false))

(fn CheckCombination
  (return (Utilities|Enum|Equal(Enum) (Variables|LockSettings|GetAnswer) (Utilities|String|Append (Utilities|String|ToString(Integer) (Variables|/Game/Programming/Blueprints/BP_LockTumbler.BP_LockTumbler_C|GetTumblerNumber (.AsBP%20Lock%20Tumbler (Utilities|Casting|CastToBP_LockTumbler (Variables|/Script/Engine.ChildActorComponent|GetChildActor (Variables|Default|GetBP_LockTumbler1)))))) (Utilities|String|ToString(Integer) (Variables|/Game/Programming/Blueprints/BP_LockTumbler.BP_LockTumbler_C|GetTumblerNumber (.AsBP%20Lock%20Tumbler (Utilities|Casting|CastToBP_LockTumbler (Variables|/Script/Engine.ChildActorComponent|GetChildActor (Variables|Default|GetBP_LockTumbler2)))))) (Utilities|String|ToString(Integer) (Variables|/Game/Programming/Blueprints/BP_LockTumbler.BP_LockTumbler_C|GetTumblerNumber (.AsBP%20Lock%20Tumbler (Utilities|Casting|CastToBP_LockTumbler (Variables|/Script/Engine.ChildActorComponent|GetChildActor (Variables|Default|GetBP_LockTumbler3)))))) (Utilities|String|ToString(Integer) (Variables|/Game/Programming/Blueprints/BP_LockTumbler.BP_LockTumbler_C|GetTumblerNumber (.AsBP%20Lock%20Tumbler (Utilities|Casting|CastToBP_LockTumbler (Variables|/Script/Engine.ChildActorComponent|GetChildActor (Variables|Default|GetBP_LockTumbler4))))))))))