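; Cable-plugging puzzle where the player drags four connectors into matching sockets, with a camera collision box handling puzzle entry and exit.
; While a connector is held, Tick traces the cursor against MouseCollisionBox, easing it toward the hit point.
; Socket overlaps snap and record connections, marking correct displays, while clicking a plugged connector clears them.
; BeginPlay pre-plugs two connectors; all-correct answers update the main display, lock connectors and disable input.
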(event OnComponentBeginOverlap(CollisionBox)
  (params (OverlappedComponent :type Primitive%20Component%20Object%20Reference) (OtherActor :type Actor%20Object%20Reference) (OtherComp :type Primitive%20Component%20Object%20Reference) (OtherBodyIndex :type Integer) (bFromSweep :type Boolean) (SweepResult :type Hit%20Result%20Structure%20%28by%20ref%29))
  ;[1 1 1] 카메라 줌 오버랩
  (CallFunction|BeginOverlapPuzzle OtherActor self (Variables|Default|GetCamera)))

(event OnComponentEndOverlap(CollisionBox)
  (params (OverlappedComponent :type Primitive%20Component%20Object%20Reference) (OtherActor :type Actor%20Object%20Reference) (OtherComp :type Primitive%20Component%20Object%20Reference) (OtherBodyIndex :type Integer))
  ;[1 1 1] 카메라 줌 오버랩
  (CallFunction|EndOverlapPuzzle OtherActor))

(event OnComponentBeginOverlap(C01_Connector-)
  (params (OverlappedComponent :type Primitive%20Component%20Object%20Reference) (OtherActor :type Actor%20Object%20Reference) (OtherComp :type Primitive%20Component%20Object%20Reference) (OtherBodyIndex :type Integer) (bFromSweep :type Boolean) (SweepResult :type Hit%20Result%20Structure%20%28by%20ref%29))
  ;[1 1 1] 단자 꽃을 시
  (CallFunction|OverlapConnector- 2 OverlappedComponent OtherComp (Variables|Default|GetDisplay3) (Variables|Default|GetC01_Connector+))
  (CallFunction|CheckAnswer))

(event OnComponentBeginOverlap(C03_Connector-)
  (params (OverlappedComponent :type Primitive%20Component%20Object%20Reference) (OtherActor :type Actor%20Object%20Reference) (OtherComp :type Primitive%20Component%20Object%20Reference) (OtherBodyIndex :type Integer) (bFromSweep :type Boolean) (SweepResult :type Hit%20Result%20Structure%20%28by%20ref%29))
  ;[1 1 1] 단자 꽃을 시
  (CallFunction|OverlapConnector- 0 OverlappedComponent OtherComp (Variables|Default|GetDisplay1) (Variables|Default|GetC03_Connector+))
  (CallFunction|CheckAnswer))

(event OnComponentBeginOverlap(C04_Connector-)
  (params (OverlappedComponent :type Primitive%20Component%20Object%20Reference) (OtherActor :type Actor%20Object%20Reference) (OtherComp :type Primitive%20Component%20Object%20Reference) (OtherBodyIndex :type Integer) (bFromSweep :type Boolean) (SweepResult :type Hit%20Result%20Structure%20%28by%20ref%29))
  ;[1 1 1] 단자 꽃을 시
  (CallFunction|OverlapConnector- 1 OverlappedComponent OtherComp (Variables|Default|GetDisplay2) (Variables|Default|GetC04_Connector+))
  (CallFunction|CheckAnswer))

(event OnComponentBeginOverlap(C02_Connector-)
  (params (OverlappedComponent :type Primitive%20Component%20Object%20Reference) (OtherActor :type Actor%20Object%20Reference) (OtherComp :type Primitive%20Component%20Object%20Reference) (OtherBodyIndex :type Integer) (bFromSweep :type Boolean) (SweepResult :type Hit%20Result%20Structure%20%28by%20ref%29))
  ;[1 1 1] 단자 꽃을 시
  (CallFunction|OverlapConnector- 3 OverlappedComponent OtherComp (Variables|Default|GetDisplay4) (Variables|Default|GetC02_Connector+))
  (CallFunction|CheckAnswer))

(event OnClicked(C01_Connector+)
  (params (TouchedComponent :type Primitive%20Component%20Object%20Reference) (ButtonPressed :type Key%20Structure :default "None"))
  ;[1 1 1] 커넥터 클릭시
  (Variables|Default|SetSelectedConnector (Variables|Default|GetC01_Connector+))
  (CallFunction|AlreadyConnected? (Variables|Default|GetDisplay3))
  (CallFunction|OnClickedConnector))

(event OnClicked(C02_Connector+)
  (params (TouchedComponent :type Primitive%20Component%20Object%20Reference) (ButtonPressed :type Key%20Structure :default "None"))
  ;[1 1 1] 커넥터 클릭시
  (Variables|Default|SetSelectedConnector (Variables|Default|GetC02_Connector+))
  (CallFunction|AlreadyConnected? (Variables|Default|GetDisplay4))
  (CallFunction|OnClickedConnector))

(event OnClicked(C03_Connector+)
  (params (TouchedComponent :type Primitive%20Component%20Object%20Reference) (ButtonPressed :type Key%20Structure :default "None"))
  ;[1 1 1] 커넥터 클릭시
  (Variables|Default|SetSelectedConnector (Variables|Default|GetC03_Connector+))
  (CallFunction|AlreadyConnected? (Variables|Default|GetDisplay1))
  (CallFunction|OnClickedConnector))

(event OnClicked(C04_Connector+)
  (params (TouchedComponent :type Primitive%20Component%20Object%20Reference) (ButtonPressed :type Key%20Structure :default "None"))
  ;[1 1 1] 커넥터 클릭시
  (Variables|Default|SetSelectedConnector (Variables|Default|GetC04_Connector+))
  (CallFunction|AlreadyConnected? (Variables|Default|GetDisplay2))
  (CallFunction|OnClickedConnector))

(event Custom|OnClickedConnector
  ;[1 1 1] 클릭 커스텀 이벤트
  (Variables|Default|SetGrabbingCable? true)
  (Physics|SetSimulatePhysics (Variables|Default|GetSelectedConnector) false))

(event EventBeginPlay
  ;[1 1 1] BeginPlay
  (CallFunction|SetBegin))

(event EventTick
  (params (DeltaSeconds :type Float%20%28single-precision%29))
  ;[1 1 1] 단자 옮기기
  (if (Variables|Default|GetGrabbingCable?)
    (CallFunction|SetSelectedConnectorLocation&Rotation (Variables|Default|GetSelectedConnector))))

(event Input|KeyboardEvents|3
  (params (Key :type Key%20Structure :default "None"))
  ;[1 1 1] Test
)

(event Input|MouseEvents|LeftMouseButton
  (params (Key :type Key%20Structure :default "None"))
  ;[1 1 1] 클릭 커스텀 이벤트
  (:Released
    (if (Variables|Default|GetGrabbingCable?)
      (Variables|Default|SetGrabbingCable? false)
      (Utilities|IsValid (Variables|Default|GetSelectedConnector)
        (:Is%20Valid
          (Physics|SetSimulatePhysics (Variables|Default|GetSelectedConnector) false)
          (Variables|Default|SetSelectedConnector 0))))))

(event Input|KeyboardEvents|4
  (params (Key :type Key%20Structure :default "None"))
  ;[1 1 1] Test
)

(event Input|KeyboardEvents|5
  (params (Key :type Key%20Structure :default "None"))
  ;[1 1 1] Test
)

(fn ConstructionScript)

(fn SetSelectedConnectorLocation&Rotation
  (params (Connector :type Static%20Mesh%20Component%20Object%20Reference))
  (bind _returnvalue (Game|GetPlayerController 0))
  (bind _selectedconnector (Variables|Default|GetSelectedConnector))
  (bind _returnvalue_2 (Transformation|GetWorldLocation _selectedconnector))
  (bind (_worldlocation _worlddirection) (Game|Player|ConvertMouseLocationToWorldSpace _returnvalue))
  (bind _outhit (Collision|LineTraceByChannel _worldlocation (+ _worldlocation (* _worlddirection (Variables|Default|GetLineTraceValue))) "TraceTypeQuery1" false 0 "None" false "(R=1.000000,G=0.000000,B=0.000000,A=1.000000)" "(R=0.000000,G=1.000000,B=0.000000,A=1.000000)" 1e+01))
  (if (== (.HitComponent (Collision|BreakHitResult _outhit)) (Variables|Default|GetMouseCollisionBox))
    (Variables|Default|SetMouseLocationInWorld (.Location (Collision|BreakHitResult _outhit)))
    ;[1 1 1] Set Selected Connector Location And Rotation
    (Transformation|SetWorldLocationAndRotation (Variables|Default|GetSelectedConnector) (+ (* (- (Variables|Default|GetMouseLocationInWorld) _returnvalue_2) (Variables|Default|GetMoveVelocity)) _returnvalue_2) (Math|Rotator|FindLookatRotation (Transformation|GetWorldLocation (Variables|Default|GetSelectedConnector)) (Variables|Default|GetMouseLocationInWorld)) false false)))

(fn OverlapConnector-
  (params (Index :type Integer) (OverlappedConnector- :type Primitive%20Component%20Object%20Reference) (OverlappedConnector+ :type Scene%20Component%20Object%20Reference) (Display :type Static%20Mesh%20Component%20Object%20Reference) (AnswerConnector+ :type Static%20Mesh%20Component%20Object%20Reference))
  (if (not (Utilities|Array|Get(acopy) (Variables|Default|GetConnected?) Index))
    (Variables|Default|SetGrabbingCable? false)
    (Transformation|SetWorldLocationAndRotation OverlappedConnector+ (+ (Transformation|GetWorldLocation OverlappedConnector-) "0.000000,0.000000,3.000000") "-90.000000,180.000000,180.000000" true false)
    (Utilities|Array|SetArrayElem (Variables|Default|GetConnected?) Index true)
    (Utilities|Map|Add (Variables|Default|GetMapTest) (Variables|Default|GetSelectedConnector) Index)
    ;[1 1 1] 정답 단자일 경우
    (if (== (Variables|Default|GetSelectedConnector) AnswerConnector+)
      (Rendering|Material|SetMaterial Display 0 "/Game/Evidence+Puzzle_Asset/EviPuzzle4_2/MM_4_2PuzzleOX_O.MM_4_2PuzzleOX_O")
      (Utilities|Array|SetArrayElem (Variables|Default|GetConnectedAnswer?) Index true))))

(fn CheckAnswer
  (bind _c04_connector_ (Variables|Default|GetC04_Connector+))
  (bind _c01_connector_ (Variables|Default|GetC01_Connector+))
  (bind _c02_connector_ (Variables|Default|GetC02_Connector+))
  (bind _c03_connector_ (Variables|Default|GetC03_Connector+))
  (for _array_element (Variables|Default|GetConnectedAnswer?)
    (if (not _array_element)
      (return)))
  (Rendering|Material|SetMaterial (Variables|Default|GetDisplayDC_C) 0 "/Game/Evidence+Puzzle_Asset/EviPuzzle4_2/MM_4_2Puzzle_OX_C.MM_4_2Puzzle_OX_C")
  (Utilities|FlowControl|Sequence
    (:then_0
      (Physics|SetSimulatePhysics _c04_connector_ false)
      (Collision|SetCollisionEnabled _c04_connector_ "NoCollision"))
    (:then_1
      (Physics|SetSimulatePhysics _c03_connector_ false)
      (Collision|SetCollisionEnabled _c03_connector_ "NoCollision"))
    (:then_2
      (Physics|SetSimulatePhysics _c02_connector_ false)
      (Collision|SetCollisionEnabled _c02_connector_ "NoCollision"))
    (:then_3
      (Physics|SetSimulatePhysics _c01_connector_ false)
      (Collision|SetCollisionEnabled _c01_connector_ "NoCollision"))
    (:then_4
      (Input|DisableInput (Game|GetPlayerController 0)))))

(fn FindIndex
  (params (Connector- :type Scene%20Component%20Object%20Reference))
  (if (== Connector- (Variables|Default|GetC01_Connector-))
    (return 0)
    (elif (== Connector- (Variables|Default|GetC02_Connector-))
      (return 1)
      (elif (== Connector- (Variables|Default|GetC03_Connector-))
        (return 2)
        (else
          (return 3))))))

(fn AlreadyConnected?
  (params (Display :type Static%20Mesh%20Component%20Object%20Reference))
  (bind _maptest (Variables|Default|GetMapTest))
  (bind _selectedconnector (Variables|Default|GetSelectedConnector))
  (bind (_value _returnvalue) (Utilities|Map|Find _maptest _selectedconnector))
  (if _returnvalue
    (Rendering|Material|SetMaterial Display 0 "/Game/Evidence+Puzzle_Asset/EviPuzzle4_2/MM_4_2PuzzleOX_X.MM_4_2PuzzleOX_X")
    (Utilities|Array|SetArrayElem (Variables|Default|GetConnected?) _value false)
    (Utilities|Array|SetArrayElem (Variables|Default|GetConnectedAnswer?) _value false)
    (Utilities|Map|Remove (Variables|Default|GetMapTest) (Variables|Default|GetSelectedConnector)))
  (return))

(fn SetBegin
  (bind _c01_connector_ (Variables|Default|GetC01_Connector+))
  (bind _c04_connector_ (Variables|Default|GetC04_Connector+))
  (Variables|Default|SetSelectedConnector _c01_connector_)
  (CallFunction|OverlapConnector- 0 (Variables|Default|GetC03_Connector-) _c01_connector_ (Variables|Default|GetDisplay1) (Variables|Default|GetC03_Connector+))
  (Variables|Default|SetSelectedConnector _c04_connector_)
  (CallFunction|OverlapConnector- 1 (Variables|Default|GetC04_Connector-) _c04_connector_ (Variables|Default|GetDisplay2) _c04_connector_)
  (Variables|Default|SetSelectedConnector 0))