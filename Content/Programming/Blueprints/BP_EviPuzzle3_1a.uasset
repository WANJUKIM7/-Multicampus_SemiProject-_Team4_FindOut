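; Zoomable evidence puzzle with four bird-picture cubes that opens a drawer when order and rotation are correct.
; Three cubes are set at BeginPlay; clicking Place4 adds the last once the item is usable, unlocking selection.
; A clicked cube lifts, rotates with 1/2 and swaps neighbours with arrows via timelines; lowering it compares concatenated state strings to the answers.
; Clicking Hint removes it, zooms out and marks the cubes solved.
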(event OnClicked(Hint)
  (params (TouchedComponent :type Primitive%20Component%20Object%20Reference) (ButtonPressed :type Key%20Structure :default "None"))
  ;[1 1 1] 퍼즐 맞춘 후
  (Components|DestroyComponent (Variables|Default|GetHint))
  (CallFunction|ZoomOutPuzzle self)
  (Variables|Default|SetTags (Variables|Default|Get태그))
  (Default|Solved (.AsBP%20Puzzle%203%201a%20Item (Utilities|Casting|CastToBP_Puzzle_3_1a_Item (Variables|/Script/Engine.ChildActorComponent|GetChildActor (Variables|Default|GetBP_Puzzle_3_1a_Item1)))))
  (Default|Solved (.AsBP%20Puzzle%203%201a%20Item (Utilities|Casting|CastToBP_Puzzle_3_1a_Item (Variables|/Script/Engine.ChildActorComponent|GetChildActor (Variables|Default|GetBP_Puzzle_3_1a_Item2)))))
  (Default|Solved (.AsBP%20Puzzle%203%201a%20Item (Utilities|Casting|CastToBP_Puzzle_3_1a_Item (Variables|/Script/Engine.ChildActorComponent|GetChildActor (Variables|Default|GetBP_Puzzle_3_1a_Item3)))))
  (Default|Solved (.AsBP%20Puzzle%203%201a%20Item (Utilities|Casting|CastToBP_Puzzle_3_1a_Item (Variables|/Script/Engine.ChildActorComponent|GetChildActor (Variables|Default|GetBP_Puzzle_3_1a_Item4))))))

(event OnComponentBeginOverlap(ZoomCollision)
  (params (OverlappedComponent :type Primitive%20Component%20Object%20Reference) (OtherActor :type Actor%20Object%20Reference) (OtherComp :type Primitive%20Component%20Object%20Reference) (OtherBodyIndex :type Integer) (bFromSweep :type Boolean) (SweepResult :type Hit%20Result%20Structure%20%28by%20ref%29))
  ;[1 1 1] ZoomIn을 하기 위한 오버랩 이벤트
  (CallFunction|BeginOverlapPuzzle OtherActor self (Variables|Default|GetCamera)))

(event OnClicked(Place4)
  (params (TouchedComponent :type Primitive%20Component%20Object%20Reference) (ButtonPressed :type Key%20Structure :default "None"))
  ;[1 1 1] 마지막 아이템 놓기
  (if (Variables|Lift|GetItemReadyToUse?)
    (Utilities|FlowControl|DoOnce false
      (:Completed
        (bind _asbp_puzzle_3_1a_item (Utilities|Casting|CastToBP_Puzzle_3_1a_Item (Variables|/Script/Engine.ChildActorComponent|GetChildActor (Variables|Default|GetBP_Puzzle_3_1a_Item4))))
        (Variables|/Game/Programming/Blueprints/BP_Puzzle_3_1a_Item.BP_Puzzle_3_1a_Item_C|SetSequence _asbp_puzzle_3_1a_item 4)
        (bind _output_get (Variables|/Game/Programming/Blueprints/BP_Puzzle_3_1a_Item.BP_Puzzle_3_1a_Item_C|SetRotationCount _asbp_puzzle_3_1a_item 2))
        (CallFunction|SetBeginRotation _output_get (Variables|/Game/Programming/Blueprints/BP_Puzzle_3_1a_Item.BP_Puzzle_3_1a_Item_C|GetItem _asbp_puzzle_3_1a_item))
        (Variables|/Game/Programming/Blueprints/BP_Puzzle_3_1a_Item.BP_Puzzle_3_1a_Item_C|SetSequenceGuess _asbp_puzzle_3_1a_item 2)
        (CallFunction|SetSecondItem (Variables|/Game/Programming/Blueprints/BP_Puzzle_3_1a_Item.BP_Puzzle_3_1a_Item_C|GetItem _asbp_puzzle_3_1a_item))
        (Collision|SetCollisionEnabled (Variables|Default|GetPlace4) "NoCollision")
        ;[1 1 1] Event BeginPlay - Click Event Binding, 아이템 3개 셋팅
        (bind _output_get_2 (Variables|Lift|SetPlacedItemsCount (+ (Variables|Lift|GetPlacedItemsCount) 1)))
        (if (== _output_get_2 4)
          (Variables|Lift|SetItemPacked? true))))))

(event OnComponentEndOverlap(ZoomCollision)
  (params (OverlappedComponent :type Primitive%20Component%20Object%20Reference) (OtherActor :type Actor%20Object%20Reference) (OtherComp :type Primitive%20Component%20Object%20Reference) (OtherBodyIndex :type Integer))
  ;[1 1 1] ZoomIn을 하기 위한 오버랩 이벤트
  (CallFunction|EndOverlapPuzzle OtherActor))

(event Custom|RightReset
  (bind _selecteditem_actor_ (Variables|Lift|GetSelectedItem%28Actor%29))
  (bind _asbp_puzzle_3_1a_item (Utilities|Casting|CastToBP_Puzzle_3_1a_Item _selecteditem_actor_))
  (bind _sequence (Variables|/Game/Programming/Blueprints/BP_Puzzle_3_1a_Item.BP_Puzzle_3_1a_Item_C|GetSequence _asbp_puzzle_3_1a_item))
  ;[1 1 1] Item 왼쪽 오른쪽 움직이기
  (Utilities|FlowControl|DoOnce false) ; enters at Reset
)

(event Custom|LiftDownReset
  (bind _selecteditem_primitive_ (Variables|Lift|GetSelectedItem%28Primitive%29))
  (bind _drawer (Variables|Default|GetDrawer))
  ;[1 1 1] LiftUp & LiftDown
  (Utilities|FlowControl|DoOnce true) ; enters at Reset
)

(event Custom|LiftDownItem
  (bind _selecteditem_primitive_ (Variables|Lift|GetSelectedItem%28Primitive%29))
  (bind _drawer (Variables|Default|GetDrawer))
  ;[1 1 1] LiftUp & LiftDown
  (if (Variables|Lift|GetLifted?)
    (Utilities|FlowControl|DoOnce true
      (:Completed
        (Variables|Lift|SetClickEventStop true)
        (Input|DisableInput (Game|GetPlayerController 0))
        (Components|MoveComponentTo _selecteditem_primitive_ (- (Variables|/Script/Engine.SceneComponent|GetRelativeLocation _selecteditem_primitive_) (Variables|Lift|GetLiftLocation)) (Variables|/Script/Engine.SceneComponent|GetRelativeRotation _selecteditem_primitive_) true true (Variables|Lift|GetLiftTime) false)
        (Variables|Lift|SetLifted? false)
        (Variables|Lift|SetClickEventStop false)
        (bind _solved_ (CallFunction|CheckAnswer))
        (if _solved_
          ;[1 1 1] 퍼즐 맞춘 후
          (Components|MoveComponentTo _drawer (+ (Variables|/Script/Engine.SceneComponent|GetRelativeLocation _drawer) "0.000000,30.000000,0.000000") "0, 0, 0" true true 0.5 false)
          (else
            (CallFunction|LiftUpReset)))))))

(event Custom|OnClickedItem3
  (params (TouchedActor :type Actor%20Object%20Reference) (ButtonPressed :type Key%20Structure :default "None"))
  ;[1 1 1] Event BeginPlay - Click Event Binding, 아이템 3개 셋팅
  (if (not (Variables|Lift|GetClickEventStop))
    (Variables|Lift|SetSelectedItem%28Actor%29 TouchedActor)
    (CallFunction|OnClickedItem (Actor|GetComponentbyClass TouchedActor "/Script/Engine.PrimitiveComponent"))))

(event Custom|RotateBackReset
  ;[1 1 1] Rotate
  (Utilities|FlowControl|DoOnce false) ; enters at Reset
)

(event Custom|RotateReset
  ;[1 1 1] Rotate
  (Utilities|FlowControl|DoOnce false) ; enters at Reset
)

(event Custom|OnClickedItem1
  (params (TouchedActor :type Actor%20Object%20Reference) (ButtonPressed :type Key%20Structure :default "None"))
  ;[1 1 1] Event BeginPlay - Click Event Binding, 아이템 3개 셋팅
  (if (not (Variables|Lift|GetClickEventStop))
    (Variables|Lift|SetSelectedItem%28Actor%29 TouchedActor)
    (CallFunction|OnClickedItem (Actor|GetComponentbyClass TouchedActor "/Script/Engine.PrimitiveComponent"))))

(event Custom|Left_Reset
  (bind _selecteditem_actor_ (Variables|Lift|GetSelectedItem%28Actor%29))
  (bind _asbp_puzzle_3_1a_item (Utilities|Casting|CastToBP_Puzzle_3_1a_Item _selecteditem_actor_))
  (bind _sequence (Variables|/Game/Programming/Blueprints/BP_Puzzle_3_1a_Item.BP_Puzzle_3_1a_Item_C|GetSequence _asbp_puzzle_3_1a_item))
  ;[1 1 1] Item 왼쪽 오른쪽 움직이기
  (Utilities|FlowControl|DoOnce false) ; enters at Reset
)

(event Custom|OnClickedItem2
  (params (TouchedActor :type Actor%20Object%20Reference) (ButtonPressed :type Key%20Structure :default "None"))
  ;[1 1 1] Event BeginPlay - Click Event Binding, 아이템 3개 셋팅
  (if (not (Variables|Lift|GetClickEventStop))
    (Variables|Lift|SetSelectedItem%28Actor%29 TouchedActor)
    (CallFunction|OnClickedItem (Actor|GetComponentbyClass TouchedActor "/Script/Engine.PrimitiveComponent"))))

(event Custom|LiftUpItem
  (bind _selecteditem_primitive_ (Variables|Lift|GetSelectedItem%28Primitive%29))
  ;[1 1 1] LiftUp & LiftDown
  (Utilities|FlowControl|DoOnce false
    (:Completed
      (if (not (Variables|Lift|GetLifted?))
        (Variables|Lift|SetLifted? true)
        (Variables|Lift|SetClickEventStop true)
        (Components|MoveComponentTo _selecteditem_primitive_ (+ (Variables|/Script/Engine.SceneComponent|GetRelativeLocation _selecteditem_primitive_) (Variables|Lift|GetLiftLocation)) (Variables|/Script/Engine.SceneComponent|GetRelativeRotation _selecteditem_primitive_) true true (Variables|Lift|GetLiftTime) false)
        (Variables|Lift|SetLiftedItem (Variables|Lift|GetSelectedItem%28Primitive%29))
        (Variables|Lift|SetClickEventStop false)
        (Input|EnableInput (Game|GetPlayerController 0))
        (CallFunction|LiftDownReset)))))

(event Custom|LiftUpReset
  (bind _selecteditem_primitive_ (Variables|Lift|GetSelectedItem%28Primitive%29))
  ;[1 1 1] LiftUp & LiftDown
  (Utilities|FlowControl|DoOnce false) ; enters at Reset
)

(event Custom|OnClickedItem4
  (params (TouchedActor :type Actor%20Object%20Reference) (ButtonPressed :type Key%20Structure :default "None"))
  ;[1 1 1] Event BeginPlay - Click Event Binding, 아이템 3개 셋팅
  (if (not (Variables|Lift|GetClickEventStop))
    (Variables|Lift|SetSelectedItem%28Actor%29 TouchedActor)
    (CallFunction|OnClickedItem (Actor|GetComponentbyClass TouchedActor "/Script/Engine.PrimitiveComponent"))))

(event EventBeginPlay
  ;[1 1 1] Event BeginPlay - Click Event Binding, 아이템 3개 셋팅
  (Utilities|FlowControl|Sequence
    (:then_0
      (EventDispatchers|BindEventtoOnClicked (.AsBP%20Puzzle%203%201a%20Item (Utilities|Casting|CastToBP_Puzzle_3_1a_Item (Variables|/Script/Engine.ChildActorComponent|GetChildActor (Variables|Default|GetBP_Puzzle_3_1a_Item1)))) (delegate Custom|OnClickedItem1)))
    (:then_1
      (EventDispatchers|BindEventtoOnClicked (.AsBP%20Puzzle%203%201a%20Item (Utilities|Casting|CastToBP_Puzzle_3_1a_Item (Variables|/Script/Engine.ChildActorComponent|GetChildActor (Variables|Default|GetBP_Puzzle_3_1a_Item2)))) (delegate Custom|OnClickedItem2)))
    (:then_2
      (EventDispatchers|BindEventtoOnClicked (Variables|/Script/Engine.ChildActorComponent|GetChildActor (Variables|Default|GetBP_Puzzle_3_1a_Item3)) (delegate Custom|OnClickedItem3)))
    (:then_3
      (EventDispatchers|BindEventtoOnClicked (.AsBP%20Puzzle%203%201a%20Item (Utilities|Casting|CastToBP_Puzzle_3_1a_Item (Variables|/Script/Engine.ChildActorComponent|GetChildActor (Variables|Default|GetBP_Puzzle_3_1a_Item4)))) (delegate Custom|OnClickedItem4)))
    (:then_4
      (Utilities|FlowControl|DoOnce false
        (:Completed
          (bind _asbp_puzzle_3_1a_item (Utilities|Casting|CastToBP_Puzzle_3_1a_Item (Variables|/Script/Engine.ChildActorComponent|GetChildActor (Variables|Default|GetBP_Puzzle_3_1a_Item1))))
          (Variables|/Game/Programming/Blueprints/BP_Puzzle_3_1a_Item.BP_Puzzle_3_1a_Item_C|SetSequence _asbp_puzzle_3_1a_item 1)
          (bind _output_get (Variables|/Game/Programming/Blueprints/BP_Puzzle_3_1a_Item.BP_Puzzle_3_1a_Item_C|SetRotationCount _asbp_puzzle_3_1a_item 4))
          (CallFunction|SetBeginRotation _output_get (Variables|/Game/Programming/Blueprints/BP_Puzzle_3_1a_Item.BP_Puzzle_3_1a_Item_C|GetItem _asbp_puzzle_3_1a_item))
          (Variables|/Game/Programming/Blueprints/BP_Puzzle_3_1a_Item.BP_Puzzle_3_1a_Item_C|SetSequenceGuess _asbp_puzzle_3_1a_item 4)
          (CallFunction|SetFourthItem (Variables|/Game/Programming/Blueprints/BP_Puzzle_3_1a_Item.BP_Puzzle_3_1a_Item_C|GetItem _asbp_puzzle_3_1a_item))
          (bind _output_get_2 (Variables|Lift|SetPlacedItemsCount (+ (Variables|Lift|GetPlacedItemsCount) 1) :!label _label))
          (if (== _output_get_2 4)
            (Variables|Lift|SetItemPacked? true)))))
    (:then_5
      (Utilities|FlowControl|DoOnce false
        (:Completed
          (bind _asbp_puzzle_3_1a_item_2 (Utilities|Casting|CastToBP_Puzzle_3_1a_Item (Variables|/Script/Engine.ChildActorComponent|GetChildActor (Variables|Default|GetBP_Puzzle_3_1a_Item2))))
          (Variables|/Game/Programming/Blueprints/BP_Puzzle_3_1a_Item.BP_Puzzle_3_1a_Item_C|SetSequence _asbp_puzzle_3_1a_item_2 2)
          (bind _output_get_3 (Variables|/Game/Programming/Blueprints/BP_Puzzle_3_1a_Item.BP_Puzzle_3_1a_Item_C|SetRotationCount _asbp_puzzle_3_1a_item_2 3))
          (CallFunction|SetBeginRotation _output_get_3 (Variables|/Game/Programming/Blueprints/BP_Puzzle_3_1a_Item.BP_Puzzle_3_1a_Item_C|GetItem _asbp_puzzle_3_1a_item_2))
          (Variables|/Game/Programming/Blueprints/BP_Puzzle_3_1a_Item.BP_Puzzle_3_1a_Item_C|SetSequenceGuess _asbp_puzzle_3_1a_item_2 3)
          (CallFunction|SetThirdItem (Variables|/Game/Programming/Blueprints/BP_Puzzle_3_1a_Item.BP_Puzzle_3_1a_Item_C|GetItem _asbp_puzzle_3_1a_item_2))
          (goto _label))))
    (:then_6
      (Utilities|FlowControl|DoOnce false
        (:Completed
          (bind _asbp_puzzle_3_1a_item_3 (Utilities|Casting|CastToBP_Puzzle_3_1a_Item (Variables|/Script/Engine.ChildActorComponent|GetChildActor (Variables|Default|GetBP_Puzzle_3_1a_Item3))))
          (Variables|/Game/Programming/Blueprints/BP_Puzzle_3_1a_Item.BP_Puzzle_3_1a_Item_C|SetSequence _asbp_puzzle_3_1a_item_3 3)
          (bind _output_get_4 (Variables|/Game/Programming/Blueprints/BP_Puzzle_3_1a_Item.BP_Puzzle_3_1a_Item_C|SetRotationCount _asbp_puzzle_3_1a_item_3 2))
          (CallFunction|SetBeginRotation _output_get_4 (Variables|/Game/Programming/Blueprints/BP_Puzzle_3_1a_Item.BP_Puzzle_3_1a_Item_C|GetItem _asbp_puzzle_3_1a_item_3))
          (Variables|/Game/Programming/Blueprints/BP_Puzzle_3_1a_Item.BP_Puzzle_3_1a_Item_C|SetSequenceGuess _asbp_puzzle_3_1a_item_3 1)
          (CallFunction|SetFirstItem (Variables|/Game/Programming/Blueprints/BP_Puzzle_3_1a_Item.BP_Puzzle_3_1a_Item_C|GetItem _asbp_puzzle_3_1a_item_3))
          (goto _label))))))

(event Input|MouseEvents|LeftMouseButton
  (params (Key :type Key%20Structure :default "None"))
  ;[1 1 1] LiftUp & LiftDown
  (:Pressed
    (CallFunction|LiftDownItem)))

(event Input|KeyboardEvents|Right
  (params (Key :type Key%20Structure :default "None"))
  (bind _selecteditem_actor_ (Variables|Lift|GetSelectedItem%28Actor%29))
  (bind _asbp_puzzle_3_1a_item (Utilities|Casting|CastToBP_Puzzle_3_1a_Item _selecteditem_actor_))
  (bind _sequence (Variables|/Game/Programming/Blueprints/BP_Puzzle_3_1a_Item.BP_Puzzle_3_1a_Item_C|GetSequence _asbp_puzzle_3_1a_item))
  ;[1 1 1] Item 왼쪽 오른쪽 움직이기
  (:Pressed
    (Variables|Lift|SetClickEventStop true)
    (Input|DisableInput (Game|GetPlayerController 0))
    (Utilities|FlowControl|DoOnce false
      (:Completed
        (if (== _sequence 4)
          (Input|EnableInput (Game|GetPlayerController 0) :!label _label)
          (Variables|Lift|SetClickEventStop false)
          (CallFunction|RightReset)
          (elif (Variables|Lift|GetLifted?)
            (CallFunction|FindNearItem (+ _sequence 1))
            (Variables|Lift|SetTempLocation (Variables|/Script/Engine.SceneComponent|GetRelativeLocation (Variables|Lift|GetSelectedItem%28Primitive%29)))
            (Variables|Lift|SetTempNearLocation (Variables|/Script/Engine.SceneComponent|GetRelativeLocation (Variables|/Script/Engine.Actor|GetRootComponent (Variables|Lift|GetNearByItem))))
            (bind _alpha (Timeline|타임라인_1 PlayFromStart)
              (:Update
                (CallFunction|MoveItem _alpha))
              (:Finished
                (CallFunction|SetItemSequence (Variables|Lift|GetSelectedItem%28Actor%29) 1)
                (CallFunction|SetItemSequence (Variables|Lift|GetNearByItem) -1)
                (goto _label)))
            (else
              (goto _label))))))))

(event Input|KeyboardEvents|1
  (params (Key :type Key%20Structure :default "None"))
  ;[1 1 1] Rotate
  (:Pressed
    (if (Variables|Lift|GetLifted?)
      (Utilities|FlowControl|DoOnce false
        (:Completed
          (Input|DisableInput (Game|GetPlayerController 0))
          (Variables|Lift|SetClickEventStop true)
          (bind _alpha (Timeline|타임라인 PlayFromStart)
            (:Update
              (Transformation|SetRelativeRotation (Variables|Lift|GetSelectedItem%28Primitive%29) (Math|Rotator|MakeRotator (+ (Variables|Lift|GetCubeRotation) _alpha) 0.0 0.0) false false))
            (:Finished
              (Variables|Lift|SetCubeRotation (+ (Variables|Lift|GetCubeRotation) _alpha))
              (CallFunction|SetRotationCount 1)
              (Variables|Lift|SetClickEventStop false)
              (Input|EnableInput (Game|GetPlayerController 0))
              (CallFunction|RotateReset))))))))

(event Input|KeyboardEvents|2
  (params (Key :type Key%20Structure :default "None"))
  ;[1 1 1] Rotate
  (:Pressed
    (if (Variables|Lift|GetLifted?)
      (Utilities|FlowControl|DoOnce false
        (:Completed
          (Input|DisableInput (Game|GetPlayerController 0))
          (Variables|Lift|SetClickEventStop true)
          (bind _alpha (Timeline|타임라인_0 PlayFromStart)
            (:Update
              (Transformation|SetRelativeRotation (Variables|Lift|GetSelectedItem%28Primitive%29) (Math|Rotator|MakeRotator (- (Variables|Lift|GetCubeRotation) _alpha) 0.0 0.0) false false))
            (:Finished
              (Variables|Lift|SetCubeRotation (- (Variables|Lift|GetCubeRotation) _alpha))
              (CallFunction|SetRotationCount -1)
              (Variables|Lift|SetClickEventStop false)
              (Input|EnableInput (Game|GetPlayerController 0))
              (CallFunction|RotateBackReset))))))))

(event Input|KeyboardEvents|Left
  (params (Key :type Key%20Structure :default "None"))
  (bind _selecteditem_actor_ (Variables|Lift|GetSelectedItem%28Actor%29))
  (bind _asbp_puzzle_3_1a_item (Utilities|Casting|CastToBP_Puzzle_3_1a_Item _selecteditem_actor_))
  (bind _sequence (Variables|/Game/Programming/Blueprints/BP_Puzzle_3_1a_Item.BP_Puzzle_3_1a_Item_C|GetSequence _asbp_puzzle_3_1a_item))
  ;[1 1 1] Item 왼쪽 오른쪽 움직이기
  (:Pressed
    (Variables|Lift|SetClickEventStop true)
    (Input|DisableInput (Game|GetPlayerController 0))
    (Utilities|FlowControl|DoOnce false
      (:Completed
        (if (== _sequence 1)
          (Input|EnableInput (Game|GetPlayerController 0) :!label _label)
          (Variables|Lift|SetClickEventStop false)
          (CallFunction|LeftReset)
          (elif (Variables|Lift|GetLifted?)
            (CallFunction|FindNearItem (- _sequence 1))
            (Variables|Lift|SetTempLocation (Variables|/Script/Engine.SceneComponent|GetRelativeLocation (Variables|Lift|GetSelectedItem%28Primitive%29)))
            (Variables|Lift|SetTempNearLocation (Variables|/Script/Engine.SceneComponent|GetRelativeLocation (Variables|/Script/Engine.Actor|GetRootComponent (Variables|Lift|GetNearByItem))))
            (bind _alpha (Timeline|타임라인_2 PlayFromStart)
              (:Update
                (CallFunction|MoveItem _alpha))
              (:Finished
                (CallFunction|SetItemSequence (Variables|Lift|GetSelectedItem%28Actor%29) -1)
                (CallFunction|SetItemSequence (Variables|Lift|GetNearByItem) 1)
                (goto _label)))
            (else
              (goto _label))))))))

(event Input|KeyboardEvents|3
  (params (Key :type Key%20Structure :default "None"))
  ;[1 1 1] 퍼즐 맞춘 후
)

(fn ConstructionScript)

(fn OnClickedItem
  (params (SelectedItem :type Primitive%20Component%20Object%20Reference))
  (if (Variables|Lift|GetItemPacked?)
    (if (not (Variables|Lift|GetLifted?))
      (Variables|Lift|SetSelectedItem%28Primitive%29 SelectedItem)
      (bind _output_get (Variables|Lift|SetCubeRotation (Math|Conversions|ToFloat(Integer) (* (- (Variables|/Game/Programming/Blueprints/BP_Puzzle_3_1a_Item.BP_Puzzle_3_1a_Item_C|GetRotationCount (.AsBP%20Puzzle%203%201a%20Item (Utilities|Casting|CastToBP_Puzzle_3_1a_Item (Variables|Lift|GetSelectedItem%28Actor%29)))) 1) 90))))
      (CallFunction|LiftUpItem))))

(fn OnClickedPlace
  (params (ToucedPlace :type Static%20Mesh%20Component%20Object%20Reference))
  (Utilities|FlowControl|DoOnce false
    (:Completed
      (Components|StaticMesh|SetStaticMesh ToucedPlace "/Engine/BasicShapes/Cube.Cube")
      (Rendering|Material|SetMaterial ToucedPlace 0 "/Engine/Functions/Engine_MaterialFunctions02/ExampleContent/GradientMap_Multi_Example.GradientMap_Multi_Example")
      (Collision|SetCollisionEnabled ToucedPlace "NoCollision"))))

(fn FindNearItem
  (params (Sequence :type Integer))
  (bind _bp_puzzle_3_1a_item2 (Variables|Default|GetBP_Puzzle_3_1a_Item2))
  (bind _bp_puzzle_3_1a_item3 (Variables|Default|GetBP_Puzzle_3_1a_Item3))
  (bind _bp_puzzle_3_1a_item1 (Variables|Default|GetBP_Puzzle_3_1a_Item1))
  (bind _childactor (Variables|/Script/Engine.ChildActorComponent|GetChildActor _bp_puzzle_3_1a_item2))
  (bind _childactor_2 (Variables|/Script/Engine.ChildActorComponent|GetChildActor _bp_puzzle_3_1a_item3))
  (bind _childactor_3 (Variables|/Script/Engine.ChildActorComponent|GetChildActor _bp_puzzle_3_1a_item1))
  (if (== Sequence (Variables|/Game/Programming/Blueprints/BP_Puzzle_3_1a_Item.BP_Puzzle_3_1a_Item_C|GetSequence (.AsBP%20Puzzle%203%201a%20Item (Utilities|Casting|CastToBP_Puzzle_3_1a_Item _childactor_3))))
    (Variables|Lift|SetNearByItem _childactor_3)
    (elif (== Sequence (Variables|/Game/Programming/Blueprints/BP_Puzzle_3_1a_Item.BP_Puzzle_3_1a_Item_C|GetSequence (.AsBP%20Puzzle%203%201a%20Item (Utilities|Casting|CastToBP_Puzzle_3_1a_Item _childactor))))
      (Variables|Lift|SetNearByItem _childactor)
      (elif (== Sequence (Variables|/Game/Programming/Blueprints/BP_Puzzle_3_1a_Item.BP_Puzzle_3_1a_Item_C|GetSequence (.AsBP%20Puzzle%203%201a%20Item (Utilities|Casting|CastToBP_Puzzle_3_1a_Item _childactor_2))))
        (Variables|Lift|SetNearByItem _childactor_2)
        (else
          (Variables|Lift|SetNearByItem (Variables|/Script/Engine.ChildActorComponent|GetChildActor (Variables|Default|GetBP_Puzzle_3_1a_Item4))))))))

(fn MoveItem
  (params (Alpha :type Float%20%28double-precision%29))
  (bind _templocation (Variables|Lift|GetTempLocation))
  (bind _tempnearlocation (Variables|Lift|GetTempNearLocation))
  (Transformation|SetRelativeLocation (Variables|Lift|GetSelectedItem%28Primitive%29) (Math|Vector|MakeVector (+ Alpha (.x _templocation)) (.y _templocation) (.z _templocation)) false false)
  (Transformation|SetRelativeLocation (Variables|/Script/Engine.Actor|GetRootComponent (Variables|Lift|GetNearByItem)) (Math|Vector|MakeVector (+ (.x _tempnearlocation) (* Alpha -1.0)) (.y _tempnearlocation) (.z _tempnearlocation)) false false))

(fn SetItemSequence
  (params (Item :type Actor%20Object%20Reference) (Right1Left-1 :type Integer))
  (bind _asbp_puzzle_3_1a_item (Utilities|Casting|CastToBP_Puzzle_3_1a_Item Item))
  (Variables|/Game/Programming/Blueprints/BP_Puzzle_3_1a_Item.BP_Puzzle_3_1a_Item_C|SetSequence _asbp_puzzle_3_1a_item (+ (Variables|/Game/Programming/Blueprints/BP_Puzzle_3_1a_Item.BP_Puzzle_3_1a_Item_C|GetSequence _asbp_puzzle_3_1a_item) Right1Left-1))
  (Variables|/Game/Programming/Blueprints/BP_Puzzle_3_1a_Item.BP_Puzzle_3_1a_Item_C|SetSequenceGuess _asbp_puzzle_3_1a_item (- (Variables|/Game/Programming/Blueprints/BP_Puzzle_3_1a_Item.BP_Puzzle_3_1a_Item_C|GetSequenceGuess _asbp_puzzle_3_1a_item) Right1Left-1))
  (return))

(fn CheckAnswer
  (bind _bp_puzzle_3_1a_item3 (Variables|Default|GetBP_Puzzle_3_1a_Item3))
  (bind _bp_puzzle_3_1a_item4 (Variables|Default|GetBP_Puzzle_3_1a_Item4))
  (bind _rotationanswer (Variables|Default|GetRotationAnswer))
  (bind _sequenceanswer (Variables|Default|GetSequenceAnswer))
  (bind _bp_puzzle_3_1a_item2 (Variables|Default|GetBP_Puzzle_3_1a_Item2))
  (bind _bp_puzzle_3_1a_item1 (Variables|Default|GetBP_Puzzle_3_1a_Item1))
  (bind _childactor (Variables|/Script/Engine.ChildActorComponent|GetChildActor _bp_puzzle_3_1a_item4))
  (bind _childactor_2 (Variables|/Script/Engine.ChildActorComponent|GetChildActor _bp_puzzle_3_1a_item3))
  (bind _childactor_3 (Variables|/Script/Engine.ChildActorComponent|GetChildActor _bp_puzzle_3_1a_item1))
  (bind _childactor_4 (Variables|/Script/Engine.ChildActorComponent|GetChildActor _bp_puzzle_3_1a_item2))
  (bind _asbp_puzzle_3_1a_item (Utilities|Casting|CastToBP_Puzzle_3_1a_Item _childactor))
  (bind _asbp_puzzle_3_1a_item_2 (Utilities|Casting|CastToBP_Puzzle_3_1a_Item _childactor_3))
  (bind _asbp_puzzle_3_1a_item_3 (Utilities|Casting|CastToBP_Puzzle_3_1a_Item _childactor_4))
  (bind _asbp_puzzle_3_1a_item_4 (Utilities|Casting|CastToBP_Puzzle_3_1a_Item _childactor_2))
  (bind _sequenceguess (Variables|/Game/Programming/Blueprints/BP_Puzzle_3_1a_Item.BP_Puzzle_3_1a_Item_C|GetSequenceGuess _asbp_puzzle_3_1a_item))
  (bind _sequenceguess_2 (Variables|/Game/Programming/Blueprints/BP_Puzzle_3_1a_Item.BP_Puzzle_3_1a_Item_C|GetSequenceGuess _asbp_puzzle_3_1a_item_4))
  (bind _rotationcount (Variables|/Game/Programming/Blueprints/BP_Puzzle_3_1a_Item.BP_Puzzle_3_1a_Item_C|GetRotationCount _asbp_puzzle_3_1a_item_4))
  (bind _rotationcount_2 (Variables|/Game/Programming/Blueprints/BP_Puzzle_3_1a_Item.BP_Puzzle_3_1a_Item_C|GetRotationCount _asbp_puzzle_3_1a_item_3))
  (bind _rotationcount_3 (Variables|/Game/Programming/Blueprints/BP_Puzzle_3_1a_Item.BP_Puzzle_3_1a_Item_C|GetRotationCount _asbp_puzzle_3_1a_item))
  (bind _rotationcount_4 (Variables|/Game/Programming/Blueprints/BP_Puzzle_3_1a_Item.BP_Puzzle_3_1a_Item_C|GetRotationCount _asbp_puzzle_3_1a_item_2))
  (bind _sequenceguess_3 (Variables|/Game/Programming/Blueprints/BP_Puzzle_3_1a_Item.BP_Puzzle_3_1a_Item_C|GetSequenceGuess _asbp_puzzle_3_1a_item_2))
  (bind _sequenceguess_4 (Variables|/Game/Programming/Blueprints/BP_Puzzle_3_1a_Item.BP_Puzzle_3_1a_Item_C|GetSequenceGuess _asbp_puzzle_3_1a_item_3))
  (bind _returnvalue (Utilities|String|ToString(Integer) _sequenceguess_3))
  (bind _returnvalue_2 (Utilities|String|ToString(Integer) _rotationcount_4))
  (bind _returnvalue_3 (Utilities|String|ToString(Integer) _rotationcount_2))
  (bind _returnvalue_4 (Utilities|String|ToString(Integer) _rotationcount))
  (bind _returnvalue_5 (Utilities|String|ToString(Integer) _rotationcount_3))
  (bind _returnvalue_6 (Utilities|String|ToString(Integer) _sequenceguess))
  (bind _returnvalue_7 (Utilities|String|ToString(Integer) _sequenceguess_2))
  (bind _returnvalue_8 (Utilities|String|ToString(Integer) _sequenceguess_4))
  (bind _returnvalue_9 (Utilities|String|Append _returnvalue _returnvalue_8 _returnvalue_7 _returnvalue_6))
  (bind _returnvalue_10 (Utilities|String|Append _returnvalue_2 _returnvalue_3 _returnvalue_4 _returnvalue_5))
  (bind _returnvalue_11 (Utilities|Enum|Equal(Enum) _returnvalue_9 _sequenceanswer))
  (bind _returnvalue_12 (Utilities|Enum|Equal(Enum) _rotationanswer _returnvalue_10))
  (bind _returnvalue_13 (and _returnvalue_11 _returnvalue_12))
  (if _returnvalue_13
    _
    (else
      _))
  (return _returnvalue_13))

(fn SetRotationCount
  (params (1or-1 :type Integer))
  (bind _selecteditem_actor_ (Variables|Lift|GetSelectedItem%28Actor%29))
  (bind _selecteditem_actor__2 (Variables|Lift|GetSelectedItem%28Actor%29))
  (bind _asbp_puzzle_3_1a_item (Utilities|Casting|CastToBP_Puzzle_3_1a_Item _selecteditem_actor_))
  (bind _asbp_puzzle_3_1a_item_2 (Utilities|Casting|CastToBP_Puzzle_3_1a_Item _selecteditem_actor__2))
  (bind _output_get (Variables|/Game/Programming/Blueprints/BP_Puzzle_3_1a_Item.BP_Puzzle_3_1a_Item_C|SetRotationCount _asbp_puzzle_3_1a_item (+ (Variables|/Game/Programming/Blueprints/BP_Puzzle_3_1a_Item.BP_Puzzle_3_1a_Item_C|GetRotationCount _asbp_puzzle_3_1a_item) 1or-1)))
  (if (== _output_get 5)
    (Variables|/Game/Programming/Blueprints/BP_Puzzle_3_1a_Item.BP_Puzzle_3_1a_Item_C|SetRotationCount _asbp_puzzle_3_1a_item_2 1)
    (elif (== _output_get 0)
      (Variables|/Game/Programming/Blueprints/BP_Puzzle_3_1a_Item.BP_Puzzle_3_1a_Item_C|SetRotationCount _asbp_puzzle_3_1a_item_2 4))))

(fn SetFirstItem
  (params (Item :type Static%20Mesh%20Component%20Object%20Reference))
  (Components|StaticMesh|SetStaticMesh Item "/Game/Programming/Blueprints/ItemCube.ItemCube")
  (Rendering|Material|SetMaterial Item 0 "/Game/Evidence+Puzzle_Asset/EviPuzzle3_1/MM_Bird7_8.MM_Bird7_8")
  (Rendering|Material|SetMaterial Item 1 "/Game/Evidence+Puzzle_Asset/EviPuzzle3_1/MM_RotateBird4_3.MM_RotateBird4_3")
  (Rendering|Material|SetMaterial Item 2 "/Game/Evidence+Puzzle_Asset/EviPuzzle3_1/MM_RotateBird1_2.MM_RotateBird1_2")
  (Rendering|Material|SetMaterial Item 3 "/Game/Evidence+Puzzle_Asset/EviPuzzle3_1/MM_Bird8_9.MM_Bird8_9"))

(fn SetSecondItem
  (params (Item :type Static%20Mesh%20Component%20Object%20Reference))
  (Components|StaticMesh|SetStaticMesh Item "/Game/Programming/Blueprints/ItemCube.ItemCube")
  (Rendering|Material|SetMaterial Item 0 "/Game/Evidence+Puzzle_Asset/EviPuzzle3_1/MM_Bird8_9.MM_Bird8_9")
  (Rendering|Material|SetMaterial Item 1 "/Game/Evidence+Puzzle_Asset/EviPuzzle3_1/MM_RotateBird3_6.MM_RotateBird3_6")
  (Rendering|Material|SetMaterial Item 2 "/Game/Evidence+Puzzle_Asset/EviPuzzle3_1/MM_RotateBird2_4.MM_RotateBird2_4")
  (Rendering|Material|SetMaterial Item 3 "/Game/Evidence+Puzzle_Asset/EviPuzzle3_1/MM_Bird9_7.MM_Bird9_7"))

(fn SetThirdItem
  (params (self2 :type Static%20Mesh%20Component%20Object%20Reference))
  (Components|StaticMesh|SetStaticMesh self2 "/Game/Programming/Blueprints/ItemCube.ItemCube")
  (Rendering|Material|SetMaterial self2 0 "/Game/Evidence+Puzzle_Asset/EviPuzzle3_1/MM_Bird9_7.MM_Bird9_7")
  (Rendering|Material|SetMaterial self2 1 "/Game/Evidence+Puzzle_Asset/EviPuzzle3_1/MM_RotateBird6_5.MM_RotateBird6_5")
  (Rendering|Material|SetMaterial self2 2 "/Game/Evidence+Puzzle_Asset/EviPuzzle3_1/MM_RotateBird3_6.MM_RotateBird3_6")
  (Rendering|Material|SetMaterial self2 3 "/Game/Evidence+Puzzle_Asset/EviPuzzle3_1/MM_Bird8_9.MM_Bird8_9"))

(fn SetFourthItem
  (params (InputPin :type Static%20Mesh%20Component%20Object%20Reference))
  (Components|StaticMesh|SetStaticMesh InputPin "/Game/Programming/Blueprints/ItemCube.ItemCube")
  (Rendering|Material|SetMaterial InputPin 0 "/Game/Evidence+Puzzle_Asset/EviPuzzle3_1/MM_Bird1_2.MM_Bird1_2")
  (Rendering|Material|SetMaterial InputPin 1 "/Game/Evidence+Puzzle_Asset/EviPuzzle3_1/MM_RotateBird5_1.MM_RotateBird5_1")
  (Rendering|Material|SetMaterial InputPin 2 "/Game/Evidence+Puzzle_Asset/EviPuzzle3_1/MM_RotateBird6_5.MM_RotateBird6_5")
  (Rendering|Material|SetMaterial InputPin 3 "/Game/Evidence+Puzzle_Asset/EviPuzzle3_1/MM_Bird7_8.MM_Bird7_8"))

(fn SetBeginRotation
  (params (RotationCount :type Integer) (SelectedItem :type Primitive%20Component%20Object%20Reference))
  (Transformation|SetRelativeRotation SelectedItem (Math|Rotator|MakeRotator (Math|Conversions|ToFloat(Integer) (* (- RotationCount 1) 90)) 0.0 0.0) false false))