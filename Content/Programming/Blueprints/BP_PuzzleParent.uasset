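; BP_PuzzleParent is a base Blueprint for puzzles that the player can look at and zoom in on.
; Lookat updates the player's HUD message and crosshair, showing a magnifier and zoom prompt until the puzzle is solved.
; ZoomOnEvent and ZoomOutEvent are inheritable defaults that print debug strings, with zoom-on also showing the puzzle's description.
; ToggleFocus prints debug text and passes the focus state to InterfaceToggleFocus.
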(event Custom|ZoomOnEvent
  (params (PlayerCharacter :type BP%20First%20Person%20Character%20Object%20Reference))
  ;[1 1 1] 상속 이벤트
  (Development|PrintString "BP_ParentPuzzle : ZoomOnEvent 상속 안 할시")
  (Default|UpdateMessage (Variables|/Game/FirstPerson/Blueprints/BP_FirstPersonCharacter.BP_FirstPersonCharacter_C|GetHUD PlayerCharacter) (Variables|Default|GetDisplayDescription) true))

(event Custom|ZoomOutEvent
  ;[1 1 1] 상속 이벤트
  (Development|PrintString "BP_ParentPuzzle : ZoomOutEvent 상속 안 할시"))

(event Custom|ToggleFocus
  (params (Focused :type Boolean))
  (Development|PrintText "ff")
  (Default|InterfaceToggleFocus self Focused))

(event EventLookat
  (params (PlayerCharacter :type BP%20First%20Person%20Character%20Object%20Reference))
  (bind _hud (Variables|/Game/FirstPerson/Blueprints/BP_FirstPersonCharacter.BP_FirstPersonCharacter_C|GetHUD PlayerCharacter))
  (bind _crosshair (Variables|/Game/FirstPerson/Blueprints/BP_FirstPersonCharacter.BP_FirstPersonCharacter_C|GetCrosshair PlayerCharacter))
  ;[1 1 1] Display Message & Update Crosshair
  (if (Variables|Default|GetSolved?)
    (Default|UpdateMessage _hud (Utilities|Text|FormatText "Solved Puzzle") true)
    (Default|UpdateCrosshair+ _crosshair)
    (else
      (Default|UpdateMessage _hud (Utilities|Text|FormatText "Press E to zoom on the puzzle") true)
      (Default|UpdateCrosshairMagnifier _crosshair))))

(fn ConstructionScript)