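; Base class for items the player can pick up, inspect up close and drop.
; Interacting attaches it to the player's ItemGrip, or starts inspection if an item is already held.
; Inspection swaps the HUD for BI_Inspection and moves input to the item for mouse-drag rotation and wheel zoom before the camera.
; Child hooks customize the reset; items named "Tarot Card" keep input disabled and defer to ItemChildEvent.
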(event Custom|ToggleFocus
  (params (Focused :type Boolean))
  ;[1 1 1] Outline
  (bind _output_get (Variables|Default|SetFocused Focused))
  (Default|InterfaceToggleFocus self _output_get))

(event Custom|ItemChildEvent
  ;[1 1 1] 상속시킬 이벤트
  (Development|PrintText "itemparent : ChildEvent"))

(event Custom|ItemChildResetLocationRotation
  ;[1 1 1] 상속시킬 이벤트
  (Development|PrintText "itemparent : ItemChildReset"))

(event Custom|EnableInputParent
  ;[1 1 1] 상속시킬 이벤트
  (Input|EnableInput (Game|GetPlayerController 0)))

(event Input|EnhancedActionEvents|EnhancedInputActionIA_Interact
  (params (ActionValue :type Boolean) (ElapsedSeconds :type Float%20%28double-precision%29) (TriggeredSeconds :type Float%20%28double-precision%29) (InputAction :type Input%20Action%20Object%20Reference :default "/Game/FirstPerson/Input/Actions/IA_Interact.IA_Interact"))
  ;[1 1 1] Inspect Input
  (CallFunction|StopInspect))

(event EventLookat
  (params (PlayerCharacter :type BP%20First%20Person%20Character%20Object%20Reference))
  ;[1 1 1] Display Message
  (Default|UpdateMessage (Variables|/Game/FirstPerson/Blueprints/BP_FirstPersonCharacter.BP_FirstPersonCharacter_C|GetHUD PlayerCharacter) (Utilities|Text|FormatText "Press F to pick up {name}" (Variables|Default|GetItemName)) false))

(event EventInteractwith
  (params (PlayerCharacter :type BP%20First%20Person%20Character%20Object%20Reference))
  ;[1 1 1] Pick Up & Inspect
  (bind _output_get (Variables|Default|SetPlayer PlayerCharacter))
  (Variables|/Game/FirstPerson/Blueprints/BP_FirstPersonCharacter.BP_FirstPersonCharacter_C|GetCurrentlyHeldItem _output_get
    (:then
      (if (Utilities|Enum|Equal(Enum) (Variables|Default|GetItemName) (Utilities|Text|MakeLiteralText "Tarot Card"))
        (CallFunction|StartInspectTarotCards)
        (else
          (CallFunction|StartInspect))))
    (:else
      (CallFunction|PickUpItem))))

(event Input|MouseEvents|MouseX
  (params (AxisValue :type Float%20%28single-precision%29))
  ;[1 1 1] Inspect Input
  ;;[1 1 1] MouseX
  (if (Variables|Default|GetRotating?)
    (Transformation|SetActorRotation (Math|Rotator|CombineRotators (Transformation|GetActorRotation) (Math|Rotator|MakeRotator 0.0 0.0 (* AxisValue -5.0))))))

(event Input|MouseEvents|MouseY
  (params (AxisValue :type Float%20%28single-precision%29))
  ;[1 1 1] Inspect Input
  ;;[1 1 1] MouseY
  (if (Variables|Default|GetRotating?)
    (Transformation|SetActorRotation (Math|Rotator|CombineRotators (Transformation|GetActorRotation) (Math|Rotator|MakeRotator (* AxisValue -5.0) 0.0 0.0)))))

(event Input|MouseEvents|LeftMouseButton
  (params (Key :type Key%20Structure :default "None"))
  ;[1 1 1] Inspect Input
  (:Pressed
    (Variables|Default|SetRotating? true))
  (:Released
    (Variables|Default|SetRotating? false)))

(event Input|MouseEvents|MouseWheelUp
  (params (Key :type Key%20Structure :default "None"))
  (bind _returnvalue (Game|GetPlayerCameraManager 0))
  ;[1 1 1] Inspect Input
  ;;[1 1 1] Mouse Wheel Up
  (:Pressed
    (bind _output_get (Variables|Default|SetZoomLevel (Math|Integer|Clamp(Integer) (+ (Variables|Default|GetZoomLevel) 1) 2 20)))
    (if (< _output_get 20)
      (Transformation|SetActorLocation (+ (Camera|GetCameraLocation _returnvalue) (* (Math|Vector|GetForwardVector (Camera|GetCameraRotation _returnvalue)) (* (Variables|Default|GetZoomLevel) 10))) false false))))

(event Input|MouseEvents|MouseWheelDown
  (params (Key :type Key%20Structure :default "None"))
  (bind _returnvalue (Game|GetPlayerCameraManager 0))
  ;[1 1 1] Inspect Input
  ;;[1 1 1] Mouse Wheel Down
  (:Pressed
    (bind _output_get (Variables|Default|SetZoomLevel (Math|Integer|Clamp(Integer) (- (Variables|Default|GetZoomLevel) 1) 2 20)))
    (if (> _output_get 1)
      (Transformation|SetActorLocation (+ (Camera|GetCameraLocation _returnvalue) (* (Math|Vector|GetForwardVector (Camera|GetCameraRotation _returnvalue)) (* (Variables|Default|GetZoomLevel) 10))) false false))))

(fn ConstructionScript)

(fn PickUpItem
  (Transformation|AttachComponentToComponent (Variables|/Game/FirstPerson/Blueprints/BP_FirstPersonCharacter.BP_FirstPersonCharacter_C|GetItemGrip (Variables|Default|GetPlayer)) "None" "SnapToTarget" "SnapToTarget" "KeepWorld" true)
  (Physics|SetSimulatePhysics (Variables|Default|GetStaticMesh) false)
  (Collision|SetCollisionEnabled (Variables|Default|GetStaticMesh) "NoCollision")
  (Variables|/Game/FirstPerson/Blueprints/BP_FirstPersonCharacter.BP_FirstPersonCharacter_C|SetCurrentlyHeldItem (Variables|Default|GetPlayer) self))

(fn StartInspect
  (bind _returnvalue (Game|GetPlayerCameraManager 0))
  (bind _returnvalue_2 (Game|GetPlayerController 0))
  (Widget|SetVisibility (Variables|/Game/FirstPerson/Blueprints/BP_FirstPersonCharacter.BP_FirstPersonCharacter_C|GetHUD (Variables|Default|GetPlayer)) "Hidden")
  (bind _returnvalue_3 (UserInterface|CreateWidget "/Game/Programming/Blueprints/BI_Inspection.BI_Inspection_C"))
  (bind _output_get (Variables|Default|SetInspectionUI _returnvalue_3))
  (UserInterface|Viewport|AddtoViewport _output_get 0)
  (Input|DisableInput (Variables|Default|GetPlayer) _returnvalue_2)
  (Input|EnableInput _returnvalue_2)
  (Transformation|SetActorLocation (+ (Camera|GetCameraLocation _returnvalue) (* (Math|Vector|GetForwardVector (Camera|GetCameraRotation _returnvalue)) (* (Variables|Default|GetZoomLevel) 10))) false false))

(fn DropItem
  (bind _returnvalue (Game|GetPlayerCameraManager 0))
  (bind _staticmesh (Variables|Default|GetStaticMesh))
  (Transformation|DetachFromActor "KeepWorld" "KeepWorld" "KeepWorld")
  (Transformation|SetActorLocation (+ (Camera|GetCameraLocation _returnvalue) (* (Math|Vector|GetForwardVector (Camera|GetCameraRotation _returnvalue)) 4e+02)) false false)
  (for _array_element (Components|GetChildrenComponents _staticmesh false)
    (Physics|SetSimulatePhysics _staticmesh true)
    (Collision|SetCollisionEnabled (Variables|Default|GetStaticMesh) "QueryAndPhysics"))
  (Development|PrintText "simulate physics"))

(fn StopInspect
  (bind _returnvalue (Game|GetPlayerController 0))
  (Input|DisableInput _returnvalue)
  (Input|EnableInput (Variables|Default|GetPlayer) _returnvalue)
  (Transformation|SetActorRelativeLocation "0, 0, 0")
  (Transformation|SetActorRelativeRotation "0, 0, 0")
  (CallFunction|ItemChildResetLocationRotation)
  (Widget|RemovefromParent (Variables|Default|GetInspectionUI))
  (Widget|SetVisibility (Variables|/Game/FirstPerson/Blueprints/BP_FirstPersonCharacter.BP_FirstPersonCharacter_C|GetHUD (Variables|Default|GetPlayer)) "Visible"))

(fn StartInspectTarotCards
  (bind _returnvalue (Game|GetPlayerCameraManager 0))
  (bind _returnvalue_2 (Game|GetPlayerController 0))
  (Widget|SetVisibility (Variables|/Game/FirstPerson/Blueprints/BP_FirstPersonCharacter.BP_FirstPersonCharacter_C|GetHUD (Variables|Default|GetPlayer)) "Hidden")
  (bind _returnvalue_3 (UserInterface|CreateWidget "/Game/Programming/Blueprints/BI_Inspection.BI_Inspection_C"))
  (bind _output_get (Variables|Default|SetInspectionUI _returnvalue_3))
  (UserInterface|Viewport|AddtoViewport _output_get 0)
  (Input|DisableInput (Variables|Default|GetPlayer) _returnvalue_2)
  (Input|DisableInput _returnvalue_2)
  (Transformation|SetActorLocation (+ (Camera|GetCameraLocation _returnvalue) (* (Math|Vector|GetForwardVector (Camera|GetCameraRotation _returnvalue)) (* (Variables|Default|GetZoomLevel) 10))) false false)
  (CallFunction|ItemChildEvent))