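; Tarot card puzzle item named "Tarot Card" that holds a stack of ten Major Arcana cards.
; Focus toggles a custom-depth outline on the Empress card only.
; The item event waits a second, then fans all cards out into two slightly askew rows with simultaneous eased component moves, calling EnableInputParent once the Fool's move completes.
; The reset event snaps every card back to its staggered stack position with zero rotation.
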(event EventBeginPlay
  ;[1 1 1] BeginPlay
  (Variables|Default|SetItemName "Tarot Card"))

(event EventInterfaceToggleFocus
  (params (Focus :type Boolean))
  ;[1 1 1] Outline
  (Rendering|SetRenderCustomDepth (Variables|Default|GetTarot_03_Empress) Focus))

(event EventItemChildEvent
  (Utilities|FlowControl|Delay 1.0)
  (Utilities|FlowControl|Sequence
    (:then_0
      ;[1 1 1] 0_Fool
      (Components|MoveComponentTo (Variables|Default|GetTarot_00_Fool) (+ (.location (Transformation|GetRelativeTransform (Variables|Default|GetTarot_00_Fool))) "-130.000000,-52.000000,0.000000") "0.000000,5.000000,0.000000" true true 0.3 false)
      (CallFunction|EnableInputParent))
    (:then_1
      ;[1 1 1] 1_Empress
      (Components|MoveComponentTo (Variables|Default|GetTarot_03_Empress) (+ (.location (Transformation|GetRelativeTransform (Variables|Default|GetTarot_03_Empress))) "-65.000000,-51.000000,0.000000") "0.000000,-12.000000,0.000000" true true 0.3 false))
    (:then_2
      ;[1 1 1] 2_Hierophant
      (Components|MoveComponentTo (Variables|Default|GetTarot_05_Hierophant) (+ (.location (Transformation|GetRelativeTransform (Variables|Default|GetTarot_05_Hierophant))) "0.000000,-70.000000,0.000000") "0.000000,7.000000,0.000000" true true 0.3 false))
    (:then_3
      ;[1 1 1] 3_Hermit
      (Components|MoveComponentTo (Variables|Default|GetTarot_09_Hermit) (+ (.location (Transformation|GetRelativeTransform (Variables|Default|GetTarot_09_Hermit))) "62.000000,-48.000000,0.000000") "0.000000,22.000000,0.000000" true true 0.3 false))
    (:then_4
      ;[1 1 1] 4_Hanged Man
      (Components|MoveComponentTo (Variables|Default|GetTarot_12_Hanged_Man) (+ (.location (Transformation|GetRelativeTransform (Variables|Default|GetTarot_12_Hanged_Man))) "130.000000,-53.000000,0.000000") "0.000000,-3.000000,0.000000" true true 0.3 false))
    (:then_5
      ;[1 1 1] 5_Devil
      (Components|MoveComponentTo (Variables|Default|GetTarot_15_Devil) (+ (.location (Transformation|GetRelativeTransform (Variables|Default|GetTarot_15_Devil))) "-130.000000,48.000000,0.000000") "0.000000,-10.000000,0.000000" true true 0.3 false))
    (:then_6
      ;[1 1 1] 6_Tower
      (Components|MoveComponentTo (Variables|Default|GetTarot_16_Tower) (+ (.location (Transformation|GetRelativeTransform (Variables|Default|GetTarot_16_Tower))) "-65.000000,52.000000,0.000000") "0.000000,-7.000000,0.000000" true true 0.3 false))
    (:then_7
      ;[1 1 1] 7_Star
      (Components|MoveComponentTo (Variables|Default|GetTarot_17_Star) (+ (.location (Transformation|GetRelativeTransform (Variables|Default|GetTarot_17_Star))) "0.000000,47.000000,0.000000") "0.000000,1.000000,0.000000" true true 0.3 false))
    (:then_8
      ;[1 1 1] 8_Moon
      (Components|MoveComponentTo (Variables|Default|GetTarot_18_Moon) (+ (.location (Transformation|GetRelativeTransform (Variables|Default|GetTarot_18_Moon))) "65.000000,62.000000,0.000000") "0.000000,3.000000,0.000000" true true 0.3 false))
    (:then_9
      ;[1 1 1] 9_World
      (Components|MoveComponentTo (Variables|Default|GetTarot_21_World) (+ (.location (Transformation|GetRelativeTransform (Variables|Default|GetTarot_21_World))) "135.000000,52.000000,0.000000") "0.000000,13.000000,0.000000" true true 0.3 false))))

(event EventItemChildResetLocationRotation
  (bind _tarot_03_empress (Variables|Default|GetTarot_03_Empress))
  (bind _tarot_00_fool (Variables|Default|GetTarot_00_Fool))
  (bind _tarot_05_hierophant (Variables|Default|GetTarot_05_Hierophant))
  (bind _tarot_09_hermit (Variables|Default|GetTarot_09_Hermit))
  (bind _tarot_12_hanged_man (Variables|Default|GetTarot_12_Hanged_Man))
  (bind _tarot_15_devil (Variables|Default|GetTarot_15_Devil))
  (bind _tarot_16_tower (Variables|Default|GetTarot_16_Tower))
  (bind _tarot_17_star (Variables|Default|GetTarot_17_Star))
  (bind _tarot_18_moon (Variables|Default|GetTarot_18_Moon))
  (bind _tarot_21_world (Variables|Default|GetTarot_21_World))
  (Utilities|FlowControl|Sequence
    (:then_0
      (Transformation|SetRelativeLocation _tarot_00_fool "0.000000,0.000000,0.000000" false false)
      (Transformation|SetRelativeRotation _tarot_00_fool "0, 0, 0" false false))
    (:then_1
      (Transformation|SetRelativeLocation _tarot_03_empress "1.000000,0.000000,-1.000000" false false)
      (Transformation|SetRelativeRotation _tarot_03_empress "0, 0, 0" false false))
    (:then_2
      (Transformation|SetRelativeLocation _tarot_05_hierophant "2.000000,0.000000,-2.000000" false false)
      (Transformation|SetRelativeRotation _tarot_05_hierophant "0, 0, 0" false false))
    (:then_3
      (Transformation|SetRelativeLocation _tarot_09_hermit "3.000000,0.000000,-3.000000" false false)
      (Transformation|SetRelativeRotation _tarot_09_hermit "0, 0, 0" false false))
    (:then_4
      (Transformation|SetRelativeLocation _tarot_12_hanged_man "4.000000,0.000000,-4.000000" false false)
      (Transformation|SetRelativeRotation _tarot_12_hanged_man "0, 0, 0" false false))
    (:then_5
      (Transformation|SetRelativeLocation _tarot_15_devil "5.000000,0.000000,-5.000000" false false)
      (Transformation|SetRelativeRotation _tarot_15_devil "0, 0, 0" false false))
    (:then_6
      (Transformation|SetRelativeLocation _tarot_16_tower "6.000000,0.000000,-6.000000" false false)
      (Transformation|SetRelativeRotation _tarot_16_tower "0, 0, 0" false false))
    (:then_7
      (Transformation|SetRelativeLocation _tarot_17_star "7.000000,0.000000,-7.000000" false false)
      (Transformation|SetRelativeRotation _tarot_17_star "0, 0, 0" false false))
    (:then_8
      (Transformation|SetRelativeLocation _tarot_18_moon "8.000000,0.000000,-8.000000" false false)
      (Transformation|SetRelativeRotation _tarot_18_moon "0, 0, 0" false false))
    (:then_9
      (Transformation|SetRelativeLocation _tarot_21_world "9.000000,0.000000,-9.000000" false false)
      (Transformation|SetRelativeRotation _tarot_21_world "0, 0, 0" false false))))

(fn ConstructionScript)