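; AC_InteractionTrace is a puzzle interaction component that detects when the player camera looks at a BP_InteractionArea.
; Each Tick it line-traces forward from the camera on Visibility, with debug drawing enabled.
; A new hit actor passes an exact class-match boolean to TraceInteractionArea, whose body is empty here.
; A miss passes false every frame but leaves the cached HitActor intact, so re-hitting that actor does not report again.
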(event EventTick
  (params (DeltaSeconds :type Float%20%28single-precision%29))
  (CallFunction|Trace))

(fn Trace
  (bind _returnvalue (Game|GetPlayerCameraManager 0))
  (bind _returnvalue_2 (Transformation|GetActorLocation _returnvalue))
  (bind (_outhit _returnvalue_3) (Collision|LineTraceByChannel _returnvalue_2 (+ _returnvalue_2 (* (Math|Vector|GetForwardVector (Transformation|GetActorRotation _returnvalue)) (Variables|Default|GetLength))) "TraceTypeQuery1" false 0 "ForDuration"))
  (if _returnvalue_3
    (if (!= (.HitActor (Collision|BreakHitResult _outhit)) (Variables|Default|GetHit%20Actor))
      (Variables|Default|SetHit%20Actor (.HitActor (Collision|BreakHitResult _outhit)))
      (CallFunction|TraceInteractionArea (== (Utilities|GetClass (.HitActor (Collision|BreakHitResult _outhit))) "/Game/Programming/Puzzle/Outline/InteractionArea/BP_InteractionArea.BP_InteractionArea_C")))
    (else
      (CallFunction|TraceInteractionArea false))))

(fn TraceInteractionArea
  (params (Trace :type Boolean)))